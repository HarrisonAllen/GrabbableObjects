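; Green rupee money item that the VR player grabs by hand and collects by dropping it into an ItemBag.
; Pickup attaches it to the grabbing hand's socket, clearing any previous hand's reference and setting the new hand's grip limit.
; Drop restores physics and, on ItemBag overlap, adds one to a VRCharacter stat and destroys the rupee.
; It can also attach to a menu as a half-scale icon that ignores pickup.
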(event EventAttachtoMenu
  (params (Angle :type Rotator :default "0, 0, 0") (Orientation :type Rotator :default "0, 0, 0") (Position :type Vector :default "0, 0, 0") (Origin :type Scene%20Component%20Object%20Reference))
  (Variables|Default|SetIsMenuIcon true)
  (Physics|SetSimulatePhysics (Variables|Default|GetOrigin) false)
  (Transformation|AttachComponentToComponent Origin "None" "SnapToTarget" "SnapToTarget" "SnapToTarget" true)
  (Transformation|SetActorScale3D "0.500000,0.500000,0.500000")
  (Transformation|SetActorRelativeRotation Angle)
  (Transformation|AddActorLocalOffset Position false false)
  (Transformation|AddActorLocalRotation Orientation false false))

(event EventPickup
  (params (AttachTo :type Skeletal%20Mesh%20Component%20Object%20Reference) (Socket :type Name :default "None"))
  (bind _returnvalue (Components|GetOwner AttachTo))
  (bind _origin (Variables|Default|GetOrigin))
  (bind _gripthresh (Variables|Default|GetGripThresh))
  (bind _returnvalue_2 (Transformation|GetAttachParent _origin))
  (bind _returnvalue_3 (Components|GetOwner _returnvalue_2))
  (if (not (Variables|Default|GetIsMenuIcon))
    (Physics|SetSimulatePhysics (Variables|Default|GetOrigin) false)
    (Utilities|FlowControl|Sequence
      (:then_0
        (if (and (!= _returnvalue_2 0) (!= _returnvalue_2 _returnvalue))
          (bind _asleft_hand (Utilities|Casting|CastToLeftHand _returnvalue_3)
            (:then
              (Variables|/Game/Blueprints/Player/Hands/LeftHand.LeftHand_C|SetAttachedActor _asleft_hand 0))
            (:CastFailed
              (bind _asright_hand (Utilities|Casting|CastToRightHand _returnvalue_3))
              (Variables|/Game/Blueprints/Player/Hands/RightHand.RightHand_C|SetAttachedActor _asright_hand 0)))))
      (:then_1
        (Transformation|AttachComponentToComponent (Variables|Default|GetOrigin) AttachTo Socket "SnapToTarget" "SnapToTarget" "KeepWorld" true)
        (bind _asleft_hand_2 (Utilities|Casting|CastToLeftHand _returnvalue)
          (:then
            (Variables|/Game/Blueprints/Player/Hands/LeftHand.LeftHand_C|SetMaxGrip _asleft_hand_2 _gripthresh))
          (:CastFailed
            (bind _asright_hand_2 (Utilities|Casting|CastToRightHand _returnvalue))
            (Variables|/Game/Blueprints/Player/Hands/RightHand.RightHand_C|SetMaxGrip _asright_hand_2 _gripthresh)))))))

(event EventDrop
  (params (Dropper :type Actor%20Object%20Reference))
  (Physics|SetSimulatePhysics (Variables|Default|GetOrigin) true)
  (Transformation|DetachFromActor "KeepWorld" "KeepWorld" "KeepWorld")
  (bind _array_element (Utilities|Array|ForEachLoopwithBreak (Collision|GetOverlappingActors "/Game/Blueprints/Player/ItemBag.ItemBag_C" :!class /Script/Engine.Actor))
    (:LoopBody
      (Utilities|Casting|CastToItemBag _array_element)
      (bind _asvrcharacter (Utilities|Casting|CastToVRCharacter (Game|Player|GetPlayerPawn 0)))
      (Default|AddStat _asvrcharacter "NewEnumerator3" 1)
      (Actor|DestroyActor))))

(fn ConstructionScript)