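; A VR bomb weapon that can be grabbed, stowed or detonated, and also serves as a scaled-down menu icon.
; Pickup attaches it to a hand and enables input, while dropping it on the lower-back spawn sends it to inventory and destroys it.
; Trigger release or fire damage starts a timeline fuse that switches materials, then explodes with radial damage.
; Explosion damage detonates it immediately, chaining bombs, with an Exploding flag preventing re-entry.
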(event Custom|Explode
  (bind _origin (Variables|Default|GetOrigin))
  (bind _returnvalue (Transformation|GetWorldTransform _origin))
  (bind (_location _rotation _scale) (Math|Transform|BreakTransform _returnvalue))
  (if (Variables|Default|GetFusing)
    (Variables|Default|SetExploding true)
    (Game|Damage|ApplyRadialDamage (Variables|Default|GetDamage) (Transformation|GetWorldLocation (Variables|Default|GetOrigin)) (Variables|Default|GetRadius) "/Game/Blueprints/DamageTypes/Explosion.Explosion_C" (Utilities|Array|MakeArray self) 0 0 true "ECC_Visibility")
    (Effects|SpawnEmitteratLocation "/Game/StarterContent/Particles/P_Explosion.P_Explosion" _location _rotation _scale)
    (Actor|DestroyActor)))

(event Custom|StartTimer
  (bind _origin (Variables|Default|GetOrigin))
  (if (not (or (Variables|Default|GetExploding) (Variables|Default|GetFusing)))
    (Variables|Default|SetFusing true)
    (bind _material (Timeline|MaterialTimeline Play)
      (:Update
        (if (>= _material 0.0)
          (Rendering|Material|SetMaterial _origin 0 "/Game/Materials/BombBlue.BombBlue")
          (else
            (Rendering|Material|SetMaterial _origin 0 "/Game/Materials/BombRed.BombRed"))))
      (:Finished
        (CallFunction|Explode)))))

(event Game|Damage|EventAnyDamage
  (params (Damage :type Float%20%28single-precision%29) (DamageType :type Damage%20Type%20Object%20Reference) (InstigatedBy :type Controller%20Object%20Reference) (DamageCauser :type Actor%20Object%20Reference))
  (bind _returnvalue (Utilities|GetClass DamageType))
  (if (not (Variables|Default|GetIsMenuIcon))
    (if (and (== _returnvalue "/Game/Blueprints/DamageTypes/Explosion.Explosion_C") (not (Variables|Default|GetExploding)))
      (Variables|Default|SetFusing true)
      (CallFunction|Explode)
      (elif (and (== _returnvalue "/Game/Blueprints/DamageTypes/Fire.Fire_C") (not (or (Variables|Default|GetExploding) (Variables|Default|GetFusing))))
        (CallFunction|StartTimer)))))

(event EventAttachtoMenu
  (params (Angle :type Rotator :default "0, 0, 0") (Orientation :type Rotator :default "0, 0, 0") (Position :type Vector :default "0, 0, 0") (Origin :type Scene%20Component%20Object%20Reference))
  (Variables|Default|SetIsMenuIcon true)
  (Physics|SetSimulatePhysics (Variables|Default|GetOrigin) false)
  (Transformation|AttachComponentToComponent Origin "None" "SnapToTarget" "SnapToTarget" "SnapToTarget" true)
  (Transformation|SetActorScale3D "0.200000,0.200000,0.200000")
  (Transformation|SetActorRelativeRotation Angle)
  (Transformation|AddActorLocalOffset Position false false)
  (Transformation|AddActorLocalOffset "-0.400000,-0.400000, 0" false false)
  (Transformation|AddActorLocalRotation Orientation false false))

(event EventPickup
  (params (AttachTo :type Skeletal%20Mesh%20Component%20Object%20Reference) (Socket :type Name :default "None"))
  (bind _returnvalue (Components|GetOwner AttachTo))
  (bind _origin (Variables|Default|GetOrigin))
  (bind _gripthresh (Variables|Default|GetGripThresh))
  (bind _returnvalue_2 (Transformation|GetAttachParent _origin))
  (bind _returnvalue_3 (Components|GetOwner _returnvalue_2))
  (if (not (Variables|Default|GetIsMenuIcon))
    (Physics|SetSimulatePhysics (Variables|Default|GetOrigin) false)
    (Input|EnableInput (Game|GetPlayerController 0))
    (Variables|Default|SetHand _returnvalue)
    (Utilities|FlowControl|Sequence
      (:then_0
        (if (and (!= _returnvalue_2 0) (!= _returnvalue_2 _returnvalue))
          (bind _asleft_hand (Utilities|Casting|CastToLeftHand _returnvalue_3)
            (:then
              (Variables|/Game/Blueprints/Player/Hands/LeftHand.LeftHand_C|SetAttachedActor _asleft_hand 0))
            (:CastFailed
              (bind _asright_hand (Utilities|Casting|CastToRightHand _returnvalue_3))
              (Variables|/Game/Blueprints/Player/Hands/RightHand.RightHand_C|SetAttachedActor _asright_hand 0)))))
      (:then_1
        (Transformation|AttachComponentToComponent (Variables|Default|GetOrigin) AttachTo Socket "SnapToTarget" "SnapToTarget" "KeepWorld" true)
        (bind _asleft_hand_2 (Utilities|Casting|CastToLeftHand _returnvalue)
          (:then
            (Variables|/Game/Blueprints/Player/Hands/LeftHand.LeftHand_C|SetMaxGrip _asleft_hand_2 _gripthresh))
          (:CastFailed
            (bind _asright_hand_2 (Utilities|Casting|CastToRightHand _returnvalue))
            (Variables|/Game/Blueprints/Player/Hands/RightHand.RightHand_C|SetMaxGrip _asright_hand_2 _gripthresh)
            (Transformation|AddActorLocalOffset "4.000000, 0, 0" false false)))))))

(event EventDrop
  (params (Dropper :type Actor%20Object%20Reference))
  (bind _self self)
  (bind _category (Variables|Default|GetCategory))
  (bind _returnvalue (Utilities|GetClass _self))
  (Input|DisableInput (Game|GetPlayerController 0))
  (Variables|Default|SetHand 0)
  (Physics|SetSimulatePhysics (Variables|Default|GetOrigin) true)
  (Transformation|DetachFromActor "KeepWorld" "KeepWorld" "KeepWorld")
  (bind _array_element (Utilities|Array|ForEachLoopwithBreak (Collision|GetOverlappingActors "/Game/Blueprints/Player/LowerBackWeaponSpawn.LowerBackWeaponSpawn_C" :!class /Script/Engine.Actor))
    (:LoopBody
      (Utilities|Casting|CastToLowerBackWeaponSpawn _array_element)
      (bind _asvrcharacter (Utilities|Casting|CastToVRCharacter (Game|Player|GetPlayerPawn 0)))
      (bind _inventory (Default|GetInventoryCategory _asvrcharacter (Variables|Default|GetCategory)))
      (bind _addednew (Default|AddItem _asvrcharacter _returnvalue 1))
      (if _addednew
        (bind _index (Utilities|FlowControl|ForLoopwithBreak 0 (Utilities|Array|LastIndex _inventory) :!label _label)
          (:LoopBody
            (bind _placed (Default|SetInventoryCategory _asvrcharacter _category _returnvalue _index))
            (if _placed
              (Default|SetEquippedCategory _asvrcharacter _category _index)
              (goto _label Break)))
          (:Completed
            (Utilities|FlowControl|Sequence :!label _label_2
              (:then_0
                (bind _asmenu_base (Utilities|Casting|CastToMenuBase (Variables|/Game/Blueprints/Player/VRCharacter.VRCharacter_C|GetMenu _asvrcharacter)))
                (Variables|/Game/Blueprints/UI_Elements/Menu/MenuBase.MenuBase_C|SetCurrentDraw _asmenu_base "NewEnumerator2"))
              (:then_1
                (Actor|DestroyActor)))))
        (else
          (goto _label_2))))))

(event Input|KeyboardEvents|MotionControllerRightTrigger
  (params (Key :type Key%20Structure))
  (:Released
    (Utilities|Casting|CastToRightHand (Variables|Default|GetHand))
    (CallFunction|StartTimer)))

(event Input|KeyboardEvents|MotionControllerLeftTrigger
  (params (Key :type Key%20Structure))
  (:Released
    (Utilities|Casting|CastToLeftHand (Variables|Default|GetHand))
    (CallFunction|StartTimer)))

(fn ConstructionScript)