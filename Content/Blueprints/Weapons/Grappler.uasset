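; Grappler is the projectile for a grapple hook weapon, reporting what it hits back to its Parent GrappleHook.
; When the projectile movement stops, it checks whether the hit actor implements the Damageable interface.
; Damageable actors trigger GrappleEnemyMessage with that actor, and anything else triggers GrappleMessage.
; A bounce halts the projectile immediately.
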(event OnProjectileStop(ProjectileMovement)
  (params (ImpactResult :type Hit%20Result%20Structure%20%28by%20ref%29))
  (bind _hitactor (Collision|BreakHitResult ImpactResult))
  (bind _parent (Variables|Default|GetParent))
  (if (Utilities|DoesObjectImplementInterface _hitactor "/Game/Blueprints/Interfaces/Damageable.Damageable_C")
    (bind _asgrapple_hook (Utilities|Casting|CastToGrappleHook _parent))
    (Class|GrapplingHook|GrappleEnemy(Message) _asgrapple_hook _hitactor)
    (else
      (bind _asgrapple_hook_2 (Utilities|Casting|CastToGrappleHook _parent))
      (Class|GrapplingHook|Grapple(Message) _asgrapple_hook_2))))

(event OnComponentHit(StaticMesh)
  (params (HitComponent :type Primitive%20Component%20Object%20Reference) (OtherActor :type Actor%20Object%20Reference) (OtherComp :type Primitive%20Component%20Object%20Reference) (NormalImpulse :type Vector :default "0, 0, 0") (Hit :type Hit%20Result%20Structure%20%28by%20ref%29)))

(event OnProjectileBounce(ProjectileMovement)
  (params (ImpactResult :type Hit%20Result%20Structure%20%28by%20ref%29) (ImpactVelocity :type Vector%20%28by%20ref%29 :default "0, 0, 0"))
  (Components|Movement|StopMovementImmediately (Variables|Default|GetProjectileMovement)))

(event EventBeginPlay)

(event Collision|EventActorBeginOverlap
  (params (OtherActor :type Actor%20Object%20Reference)))

(event EventTick
  (params (DeltaSeconds :type Float%20%28single-precision%29)))

(fn ConstructionScript)