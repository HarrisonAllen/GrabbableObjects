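; VR torch weapon that can be held in either hand, swung as a blunt weapon, lit by fire, or shown as a miniature menu icon.
; Pickup attaches it to a hand and sets grip; Drop restores physics and stows it in inventory over a BackWeaponSpawn.
; Tick applies blunt damage to overlapping Damageables when HitBox moves fast.
; Fire damage lights it, starting looped radial fire damage; the extinguish logic is unconnected.
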(event OnComponentBeginOverlap(BurnBox)
  (params (OverlappedComponent :type Primitive%20Component%20Object%20Reference) (OtherActor :type Actor%20Object%20Reference) (OtherComp :type Primitive%20Component%20Object%20Reference) (OtherBodyIndex :type Integer) (bFromSweep :type Boolean) (SweepResult :type Hit%20Result%20Structure%20%28by%20ref%29))
  (if (and (Variables|Default|GetOnFire) (not (Variables|Default|GetIsMenuIcon)))
    (CallFunction|Burn)))

(event Game|Damage|EventAnyDamage
  (params (Damage :type Float%20%28single-precision%29) (DamageType :type Damage%20Type%20Object%20Reference) (InstigatedBy :type Controller%20Object%20Reference) (DamageCauser :type Actor%20Object%20Reference))
  (if (not (Variables|Default|GetIsMenuIcon))
    (if (== (Utilities|GetClass DamageType) "/Game/Blueprints/DamageTypes/Fire.Fire_C")
      (if (not (Variables|Default|GetOnFire))
        (Rendering|Material|SetMaterial (Variables|Default|GetBurnPart) 0 "/Game/Materials/GlowyTorch.GlowyTorch")
        (Rendering|SetVisibility (Variables|Default|GetPointLight) true false)
        (Utilities|Time|SetTimerbyFunctionName 0 "Burn" 0.5 true)
        (Variables|Default|SetOnFire true)))))

(event EventAttachtoMenu
  (params (Angle :type Rotator :default "0, 0, 0") (Orientation :type Rotator :default "0, 0, 0") (Position :type Vector :default "0, 0, 0") (Origin :type Scene%20Component%20Object%20Reference))
  (Variables|Default|SetIsMenuIcon true)
  (Physics|SetSimulatePhysics (Variables|Default|GetOrigin) false)
  (Transformation|AttachComponentToComponent Origin "None" "SnapToTarget" "SnapToTarget" "SnapToTarget" true)
  (Transformation|SetActorScale3D "0.100000,0.100000,0.100000")
  (Transformation|SetActorRelativeRotation Angle)
  (Transformation|AddActorLocalOffset Position false false)
  (Transformation|AddActorLocalRotation Orientation false false)
  (Transformation|AddActorLocalOffset (* (Variables|/Script/Engine.SceneComponent|GetRelativeLocation (Variables|Default|GetMiddle)) (Transformation|GetActorScale3D) "-1.000000,-1.000000,-1.000000") false false))

(event EventTick
  (params (DeltaSeconds :type Float%20%28single-precision%29))
  (bind _hitbox (Variables|Default|GetHitBox))
  (bind _hitbox_2 (Variables|Default|GetHitBox))
  (bind _returnvalue (Transformation|GetWorldLocation _hitbox_2))
  (if (not (Variables|Default|GetIsMenuIcon))
    (bind _returnvalue_2 (Physics|GetPhysicsLinearVelocity _hitbox "None"))
    (if (Math|Boolean|ORBoolean (>= (Math|Float|Absolute(Float) (.X (Math|Vector|BreakVector (Math|Vector|UnrotateVector _returnvalue_2 (Transformation|GetWorldRotation _hitbox))))) 2e+02) (>= (Math|Float|Absolute(Float) (.Y (Math|Vector|BreakVector (Math|Vector|UnrotateVector _returnvalue_2 (Transformation|GetWorldRotation _hitbox))))) 2e+02) (>= (Math|Float|Absolute(Float) (.Z (Math|Vector|BreakVector (Math|Vector|UnrotateVector _returnvalue_2 (Transformation|GetWorldRotation _hitbox))))) 2e+02))
      (Variables|Default|SetThisDamage (Variables|Default|GetBluntDamage))
      (Variables|Default|SetDamageType "/Game/Blueprints/DamageTypes/Blunt.Blunt_C")
      (for _array_element (Collision|GetOverlappingActors (Variables|Default|GetHitBox) 0 :!class /Script/Engine.PrimitiveComponent)
        (if (Utilities|DoesObjectImplementInterface _array_element "/Game/Blueprints/Interfaces/Damageable.Damageable_C")
          (Game|Damage|ApplyPointDamage _array_element (Variables|Default|GetThisDamage) (- (Transformation|GetActorLocation _array_element) _returnvalue) (Collision|MakeHitResult false false 0.0 0.0 _returnvalue _returnvalue (- (Transformation|GetActorLocation _array_element) _returnvalue) (- (Transformation|GetActorLocation _array_element) _returnvalue) 0 _array_element) 0 self (Variables|Default|GetDamageType)))))))

(event EventDrop
  (params (Dropper :type Actor%20Object%20Reference))
  (bind _category (Variables|Default|GetCategory))
  (Physics|SetSimulatePhysics (Variables|Default|GetOrigin) true)
  (Transformation|DetachFromActor "KeepWorld" "KeepWorld" "KeepWorld")
  (bind _array_element (Utilities|Array|ForEachLoopwithBreak (Collision|GetOverlappingActors "/Game/Blueprints/Player/BackWeaponSpawn.BackWeaponSpawn_C" :!class /Script/Engine.Actor))
    (:LoopBody
      (Utilities|Casting|CastToBackWeaponSpawn _array_element)
      (bind _asvrcharacter (Utilities|Casting|CastToVRCharacter (Game|Player|GetPlayerPawn 0)))
      (bind _inventory (Default|GetInventoryCategory _asvrcharacter (Variables|Default|GetCategory)))
      (bind _index (Utilities|FlowControl|ForLoopwithBreak 0 (Utilities|Array|LastIndex _inventory) :!label _label)
        (:LoopBody
          (bind _placed (Default|SetInventoryCategory _asvrcharacter _category (Utilities|GetClass self) _index))
          (if _placed
            (Default|SetEquippedCategory _asvrcharacter _category _index)
            (Actor|DestroyActor)
            (goto _label Break)))
        (:Completed
          (bind _asmenu_base (Utilities|Casting|CastToMenuBase (Variables|/Game/Blueprints/Player/VRCharacter.VRCharacter_C|GetMenu _asvrcharacter)))
          (Variables|/Game/Blueprints/UI_Elements/Menu/MenuBase.MenuBase_C|SetCurrentDraw _asmenu_base "NewEnumerator2"))))))

(event EventPickup
  (params (AttachTo :type Skeletal%20Mesh%20Component%20Object%20Reference) (Socket :type Name :default "None"))
  (bind _returnvalue (Components|GetOwner AttachTo))
  (bind _origin (Variables|Default|GetOrigin))
  (bind _gripthresh (Variables|Default|GetGripThresh))
  (bind _returnvalue_2 (Transformation|GetAttachParent _origin))
  (bind _returnvalue_3 (Components|GetOwner _returnvalue_2))
  (if (not (Variables|Default|GetIsMenuIcon))
    (Physics|SetSimulatePhysics (Variables|Default|GetOrigin) false)
    (Utilities|FlowControl|Sequence
      (:then_0
        (if (and (!= _returnvalue_2 0) (!= _returnvalue_2 _returnvalue))
          (bind _asleft_hand (Utilities|Casting|CastToLeftHand _returnvalue_3)
            (:then
              (Variables|/Game/Blueprints/Player/Hands/LeftHand.LeftHand_C|SetAttachedActor _asleft_hand 0))
            (:CastFailed
              (bind _asright_hand (Utilities|Casting|CastToRightHand _returnvalue_3))
              (Variables|/Game/Blueprints/Player/Hands/RightHand.RightHand_C|SetAttachedActor _asright_hand 0)))))
      (:then_1
        (Transformation|AttachComponentToComponent (Variables|Default|GetOrigin) AttachTo Socket "SnapToTarget" "SnapToTarget" "KeepWorld" true)
        (bind _asleft_hand_2 (Utilities|Casting|CastToLeftHand _returnvalue)
          (:then
            (Variables|/Game/Blueprints/Player/Hands/LeftHand.LeftHand_C|SetMaxGrip _asleft_hand_2 _gripthresh))
          (:CastFailed
            (bind _asright_hand_2 (Utilities|Casting|CastToRightHand _returnvalue))
            (Variables|/Game/Blueprints/Player/Hands/RightHand.RightHand_C|SetMaxGrip _asright_hand_2 _gripthresh)))))))

(fn ConstructionScript)

(fn Burn
  (Game|Damage|ApplyRadialDamage (Variables|Default|GetDamage) (Transformation|GetWorldLocation (Variables|Default|GetBurnBox)) (Variables|Default|GetRadius) "/Game/Blueprints/DamageTypes/Fire.Fire_C" 0 self 0 true "ECC_WorldStatic"))