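; Two-handed VR bow: the first hand holds it, the second pulls the string, and dropping it over the back slot stores it in inventory.
; Tick clamps the draw to the grabbing hand, positions the nocked arrow, and on release launches it with draw-scaled velocity and damage.
; The string is rebuilt every tick from two spline meshes.
; Fast swings deal blunt damage through hitboxes; a scaled-down copy serves as a menu icon.
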(event EventPickup
  (params (AttachTo :type Skeletal%20Mesh%20Component%20Object%20Reference) (Socket :type Name :default "None"))
  (bind _returnvalue (Components|GetOwner AttachTo))
  (bind _origin (Variables|Default|GetOrigin))
  (bind _gripthresh (Variables|Default|GetGripThresh))
  (bind _stringgripthresh (Variables|Default|GetStringGripThresh))
  (bind _returnvalue_2 (Transformation|GetAttachParent _origin))
  (bind _returnvalue_3 (Components|GetOwner _returnvalue_2))
  (if (not (Variables|Default|GetIsMenuIcon))
    (if (== (Variables|Default|GetSupport) 0)
      (Physics|SetSimulatePhysics (Variables|Default|GetOrigin) false)
      (Utilities|FlowControl|Sequence
        (:then_0
          (if (and (!= _returnvalue_2 0) (!= _returnvalue_2 _returnvalue))
            (bind _asleft_hand (Utilities|Casting|CastToLeftHand _returnvalue_3)
              (:then
                (Variables|/Game/Blueprints/Player/Hands/LeftHand.LeftHand_C|SetAttachedActor _asleft_hand 0))
              (:CastFailed
                (bind _asright_hand (Utilities|Casting|CastToRightHand _returnvalue_3))
                (Variables|/Game/Blueprints/Player/Hands/RightHand.RightHand_C|SetAttachedActor _asright_hand 0)))))
        (:then_1
          (Transformation|AttachComponentToComponent (Variables|Default|GetOrigin) AttachTo Socket "SnapToTarget" "SnapToTarget" "KeepWorld" true)
          (Variables|Default|SetSupport _returnvalue)
          (bind _asleft_hand_2 (Utilities|Casting|CastToLeftHand _returnvalue)
            (:then
              (Variables|/Game/Blueprints/Player/Hands/LeftHand.LeftHand_C|SetMaxGrip _asleft_hand_2 _gripthresh))
            (:CastFailed
              (bind _asright_hand_2 (Utilities|Casting|CastToRightHand _returnvalue))
              (Variables|/Game/Blueprints/Player/Hands/RightHand.RightHand_C|SetMaxGrip _asright_hand_2 _gripthresh)))))
      (else
        (bind _output_get (Variables|Default|SetStringGrabber (Components|GetOwner AttachTo)))
        (bind _asleft_hand_3 (Utilities|Casting|CastToLeftHand _output_get)
          (:then
            (Variables|Default|SetSocketName "l_string_socket")
            (Variables|/Game/Blueprints/Player/Hands/LeftHand.LeftHand_C|SetMaxGrip _asleft_hand_3 _stringgripthresh))
          (:CastFailed
            (bind _asright_hand_3 (Utilities|Casting|CastToRightHand _output_get))
            (Variables|Default|SetSocketName "r_string_socket")
            (Variables|/Game/Blueprints/Player/Hands/RightHand.RightHand_C|SetMaxGrip _asright_hand_3 _stringgripthresh)))))))

(event EventBeginPlay
  (CallFunction|ResetString))

(event EventAttachtoMenu
  (params (Angle :type Rotator :default "0, 0, 0") (Orientation :type Rotator :default "0, 0, 0") (Position :type Vector :default "0, 0, 0") (Origin :type Scene%20Component%20Object%20Reference))
  (Variables|Default|SetIsMenuIcon true)
  (Physics|SetSimulatePhysics (Variables|Default|GetOrigin) false)
  (Transformation|AttachComponentToComponent Origin "None" "SnapToTarget" "SnapToTarget" "SnapToTarget" true)
  (Transformation|SetActorScale3D "0.100000,0.100000,0.100000")
  (Transformation|SetActorRelativeRotation Angle)
  (Transformation|AddActorLocalOffset Position false false)
  (Transformation|AddActorLocalRotation Orientation false false)
  (Transformation|AddActorLocalOffset (* (Variables|/Script/Engine.SceneComponent|GetRelativeLocation (Variables|Default|GetMiddle)) (Transformation|GetActorScale3D) "-1.000000,-1.000000,-1.000000") false false))

(event EventRequestAttach
  (params (Arrow :type Actor%20Object%20Reference) (Owner :type Actor%20Object%20Reference))
  (bind _stringgripthresh (Variables|Default|GetStringGripThresh))
  (Variables|Default|SetArrow Arrow)
  (bind _output_get (Variables|Default|SetStringGrabber Owner))
  (bind _asleft_hand (Utilities|Casting|CastToLeftHand _output_get)
    (:then
      (Variables|Default|SetSocketName "l_string_socket")
      (Variables|/Game/Blueprints/Player/Hands/LeftHand.LeftHand_C|SetMaxGrip _asleft_hand _stringgripthresh)
      (Variables|/Game/Blueprints/Player/Hands/LeftHand.LeftHand_C|SetAttachedActor _asleft_hand self))
    (:CastFailed
      (bind _asright_hand (Utilities|Casting|CastToRightHand _output_get))
      (Variables|Default|SetSocketName "r_string_socket")
      (Variables|/Game/Blueprints/Player/Hands/RightHand.RightHand_C|SetMaxGrip _asright_hand _stringgripthresh)
      (Variables|/Game/Blueprints/Player/Hands/RightHand.RightHand_C|SetAttachedActor _asright_hand self))))

(event EventTick
  (params (DeltaSeconds :type Float%20%28single-precision%29))
  (bind _stringmidorigin (Variables|Default|GetStringMidOrigin))
  (bind _stringmid (Variables|Default|GetStringMid))
  (bind _hitbox (Variables|Default|GetHitBox))
  (bind _hitbox_2 (Variables|Default|GetHitBox))
  (bind _stringgrabber (Variables|Default|GetStringGrabber))
  (bind _stringmid_2 (Variables|Default|GetStringMid))
  (bind _overlaps (Variables|Default|GetOverlaps))
  (bind _returnvalue (Transformation|GetWorldLocation _stringmidorigin))
  (bind _returnvalue_2 (Transformation|GetWorldLocation _hitbox_2))
  (bind _relativelocation (Variables|/Script/Engine.SceneComponent|GetRelativeLocation _stringmid))
  (bind (_x _y _z) (Math|Vector|BreakVector _relativelocation))
  (Utilities|FlowControl|Sequence
    (:then_0
      (bind _asleft_hand (Utilities|Casting|CastToLeftHand _stringgrabber)
        (:then
          (Variables|Default|SetSocketLocation (Transformation|GetSocketLocation (Variables|/Game/Blueprints/Player/Hands/LeftHand.LeftHand_C|Getl_hand_skeletal_lowres _asleft_hand) (Variables|Default|GetSocketName)))
          (Variables|Default|SetLengthOfDraw (Math|Float|Clamp(Float) (Math|Vector|VectorLength (- _returnvalue (Variables|Default|GetSocketLocation))) 0.0 (Variables|Default|GetDrawDistance)) :!label _label)
          (Transformation|SetWorldLocation _stringmid (- _returnvalue (* (Math|Vector|Normalize (- _returnvalue (Variables|Default|GetSocketLocation))) (Math|Float|Clamp(Float) (Math|Vector|VectorLength (- _returnvalue (Variables|Default|GetSocketLocation))) 0.0 (Variables|Default|GetDrawDistance)))) false false)
          (Transformation|SetRelativeLocation _stringmid (Math|Vector|MakeVector (Math|Float|Clamp(Float) _x -1.0) _y (Math|Float|Clamp(Float) _z (* (Variables|Default|GetDrawDistance) -1.0) 0.0)) false false))
        (:CastFailed
          (bind _asright_hand (Utilities|Casting|CastToRightHand _stringgrabber)
            (:then
              (Variables|Default|SetSocketLocation (Transformation|GetSocketLocation (Variables|/Game/Blueprints/Player/Hands/RightHand.RightHand_C|Getr_hand_skeletal_lowres _asright_hand) (Variables|Default|GetSocketName)))
              (goto _label))
            (:CastFailed
              (Utilities|FlowControl|Sequence
                (:then_0
                  (if (!= (Variables|Default|GetArrow) 0)
                    (Class|Arrow|LaunchwithVelocityandDamage(Message) (Variables|Default|GetArrow) (* (* (Variables|Default|GetLaunchVelocity) (/ (Variables|Default|GetLengthOfDraw) (Variables|Default|GetDrawDistance))) (* (Variables|Default|GetLaunchVelocity) (/ (Variables|Default|GetLengthOfDraw) (Variables|Default|GetDrawDistance)))) (* (* (/ (Variables|Default|GetLengthOfDraw) (Variables|Default|GetDrawDistance)) (Variables|Default|GetArrowDamage)) (* (/ (Variables|Default|GetLengthOfDraw) (Variables|Default|GetDrawDistance)) (Variables|Default|GetArrowDamage))))
                    (Variables|Default|SetArrow 0)))
                (:then_1
                  (if (Variables|Default|GetReadyToFall)
                    (Variables|Default|SetReadyToFall false)
                    (Transformation|SetRelativeLocation _stringmid_2 (* (Variables|/Script/Engine.SceneComponent|GetRelativeLocation _stringmid_2) (Variables|Default|GetFallback)) false false)
                    (Utilities|FlowControl|Delay (Variables|Default|GetFallbackDelay))
                    (Variables|Default|SetReadyToFall true)))))))))
    (:then_1
      (CallFunction|DrawString))
    (:then_2
      (CallFunction|AttachArrow))
    (:then_3
      (if (not (Variables|Default|GetIsMenuIcon))
        (bind _returnvalue_3 (Physics|GetPhysicsLinearVelocity _hitbox "None"))
        (if (Math|Boolean|ORBoolean (>= (Math|Float|Absolute(Float) (.X (Math|Vector|BreakVector (Math|Vector|UnrotateVector _returnvalue_3 (Transformation|GetWorldRotation _hitbox))))) 2e+02) (>= (Math|Float|Absolute(Float) (.Y (Math|Vector|BreakVector (Math|Vector|UnrotateVector _returnvalue_3 (Transformation|GetWorldRotation _hitbox))))) 2e+02) (>= (Math|Float|Absolute(Float) (.Z (Math|Vector|BreakVector (Math|Vector|UnrotateVector _returnvalue_3 (Transformation|GetWorldRotation _hitbox))))) 2e+02))
          (Variables|Default|SetThisDamage (Variables|Default|GetBluntDamage))
          (Variables|Default|SetDamageType "/Game/Blueprints/DamageTypes/Blunt.Blunt_C")
          (Utilities|Array|Clear _overlaps)
          (Utilities|Array|AppendArray _overlaps (Collision|GetOverlappingActors (Variables|Default|GetHitBox) 0 :!class /Script/Engine.PrimitiveComponent))
          (Utilities|Array|AppendArray _overlaps (Collision|GetOverlappingActors (Variables|Default|GetHitBox2) 0 :!class /Script/Engine.PrimitiveComponent))
          (Utilities|Array|AppendArray _overlaps (Collision|GetOverlappingActors (Variables|Default|GetHitBox3) 0 :!class /Script/Engine.PrimitiveComponent))
          (for _array_element _overlaps
            (if (Utilities|DoesObjectImplementInterface _array_element "/Game/Blueprints/Interfaces/Damageable.Damageable_C")
              (Game|Damage|ApplyPointDamage _array_element (Variables|Default|GetThisDamage) (- (Transformation|GetActorLocation _array_element) _returnvalue_2) (Collision|MakeHitResult false false 0.0 0.0 _returnvalue_2 _returnvalue_2 (- (Transformation|GetActorLocation _array_element) _returnvalue_2) (- (Transformation|GetActorLocation _array_element) _returnvalue_2) 0 _array_element) 0 self (Variables|Default|GetDamageType)))))))))

(event EventDrop
  (params (Dropper :type Actor%20Object%20Reference))
  (bind _category (Variables|Default|GetCategory))
  (if (== Dropper (Variables|Default|GetSupport))
    (Variables|Default|SetSupport 0)
    (CallFunction|ResetString)
    (Physics|SetSimulatePhysics (Variables|Default|GetOrigin) true)
    (Transformation|DetachFromActor "KeepWorld" "KeepWorld" "KeepWorld")
    (bind _array_element (Utilities|Array|ForEachLoopwithBreak (Collision|GetOverlappingActors "/Game/Blueprints/Player/BackWeaponSpawn.BackWeaponSpawn_C" :!class /Script/Engine.Actor))
      (:LoopBody
        (Utilities|Casting|CastToBackWeaponSpawn _array_element)
        (bind _asvrcharacter (Utilities|Casting|CastToVRCharacter (Game|Player|GetPlayerPawn 0)))
        (bind _inventory (Default|GetInventoryCategory _asvrcharacter (Variables|Default|GetCategory)))
        (bind _index (Utilities|FlowControl|ForLoopwithBreak 0 (Utilities|Array|LastIndex _inventory) :!label _label)
          (:LoopBody
            (bind _placed (Default|SetInventoryCategory _asvrcharacter _category (Utilities|GetClass self) _index))
            (if _placed
              (Default|SetEquippedCategory _asvrcharacter _category _index)
              (Actor|DestroyActor)
              (goto _label Break)))
          (:Completed
            (bind _asmenu_base (Utilities|Casting|CastToMenuBase (Variables|/Game/Blueprints/Player/VRCharacter.VRCharacter_C|GetMenu _asvrcharacter)))
            (Variables|/Game/Blueprints/UI_Elements/Menu/MenuBase.MenuBase_C|SetCurrentDraw _asmenu_base "NewEnumerator2")))))
    (else
      (Variables|Default|SetStringGrabber 0))))

(fn ConstructionScript)

(fn DrawString
  (bind _returnvalue (Math|Transform|MakeTransform "0, 0, 0"))
  (bind _string (Variables|Default|GetString))
  (bind _origin (Variables|Default|GetOrigin))
  (bind _string_2 (Variables|Default|GetString))
  (bind _string_3 (Variables|Default|GetString))
  (bind _string_4 (Variables|Default|GetString))
  (bind _returnvalue_2 (Transformation|GetWorldScale _origin))
  (bind (_x _y) (Math|Vector|BreakVector _returnvalue_2))
  (bind _returnvalue_3 (/ _x 2.0))
  (bind _returnvalue_4 (/ _y 2.0))
  (bind _returnvalue_5 (Math|Vector2D|MakeVector2D _returnvalue_3 _returnvalue_4))
  (CallFunction|ClearString)
  (Spline|AddSplinePoint _string (Transformation|GetWorldLocation (Variables|Default|GetStringTop)) "Local" true)
  (Spline|AddSplinePoint _string (Transformation|GetWorldLocation (Variables|Default|GetStringMid)) "Local" true)
  (Spline|AddSplinePoint _string (Transformation|GetWorldLocation (Variables|Default|GetStringBot)) "Local" true)
  (for _index (range 0 (Spline|GetNumberOfSplinePoints _string))
    (Spline|SetSplinePointType _string_2 _index "CurveClamped" true)
    (Spline|SetTangentsatSplinePoint _string_2 _index (* (Spline|GetTangentatSplinePoint _string_2 _index "Local") (Variables|Default|GetStringBendiness)) (* (Spline|GetTangentatSplinePoint _string_2 _index "Local") (Variables|Default|GetStringBendiness)) "Local" true))
  (bind _returnvalue_6 (AddComponent|AddSplineMeshComponent true _returnvalue))
  (Utilities|Array|Add (Variables|Default|GetSplineMeshes) _returnvalue_6)
  (SplineMesh|SetStartandEnd _returnvalue_6 (Transformation|GetWorldLocation (Variables|Default|GetStringTop)) (Spline|GetTangentatSplinePoint _string_4 0 "Local") (Transformation|GetWorldLocation (Variables|Default|GetStringMid)) (Spline|GetTangentatSplinePoint _string_4 1 "Local") true :!class /Script/Engine.SplineMeshComponent)
  (bind _returnvalue_7 (AddComponent|AddSplineMeshComponent true _returnvalue))
  (Utilities|Array|Add (Variables|Default|GetSplineMeshes) _returnvalue_7)
  (SplineMesh|SetStartandEnd _returnvalue_7 (Transformation|GetWorldLocation (Variables|Default|GetStringMid)) (Spline|GetTangentatSplinePoint _string_3 1 "Local") (Transformation|GetWorldLocation (Variables|Default|GetStringBot)) (Spline|GetTangentatSplinePoint _string_3 2 "Local") true :!class /Script/Engine.SplineMeshComponent)
  (for _array_element (Variables|Default|GetSplineMeshes)
    (SplineMesh|SetStartScale _array_element _returnvalue_5 true :!class /Script/Engine.SplineMeshComponent)
    (SplineMesh|SetEndScale _array_element _returnvalue_5 true :!class /Script/Engine.SplineMeshComponent)))

(fn ClearString
  (bind _splinemeshes (Variables|Default|GetSplineMeshes))
  (Components|DestroyComponent _splinemeshes)
  (Utilities|Array|Clear _splinemeshes)
  (Spline|ClearSplinePoints (Variables|Default|GetString) true))

(fn ResetString
  (Transformation|SetRelativeLocation (Variables|Default|GetStringMid) "0, 0, 0" false false)
  (Variables|Default|SetStringGrabber 0))

(fn AttachArrow
  (if (!= (Variables|Default|GetArrow) 0)
    (Utilities|Casting|CastToLeftHand (Variables|Default|GetStringGrabber)
      (:then
        (Class|Arrow|SendAttachPoints(Message) (Variables|Default|GetArrow) (Transformation|GetWorldLocation (Variables|Default|GetStringMid)) (Transformation|GetWorldLocation (Variables|Default|GetRightNotch)) (Math|Rotator|MakeRotator (.Roll (Math|Rotator|BreakRotator (Transformation|GetWorldRotation (Variables|Default|GetArrowRotation)))) 0.0 0.0)))
      (:CastFailed
        (Utilities|Casting|CastToRightHand (Variables|Default|GetStringGrabber))
        (Class|Arrow|SendAttachPoints(Message) (Variables|Default|GetArrow) (Transformation|GetWorldLocation (Variables|Default|GetStringMid)) (Transformation|GetWorldLocation (Variables|Default|GetLeftNotch)) (Math|Rotator|MakeRotator (.Roll (Math|Rotator|BreakRotator (Transformation|GetWorldRotation (Variables|Default|GetArrowRotation)))) 0.0 0.0))))))