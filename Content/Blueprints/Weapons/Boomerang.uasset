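; VR boomerang weapon that slashes Damageable actors on fast swings or in flight, and doubles as a menu icon.
; Pickup attaches it to a hand with a camera-attached reticule; release throws it if slashing, otherwise drops it or stows it in lower-back inventory.
; Throws follow a runtime spline loop from camera aim, mirrored per hand, via timeline and RotatingMovement.
; A grab sphere is active until it hits static world or finishes, then falls.
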(event Custom|Throw
  (bind _returnvalue (Game|GetPlayerCameraManager 0))
  (bind _sweepangle (Variables|Default|GetSweepAngle))
  (bind _rotationspeed (Variables|Default|GetRotationSpeed))
  (bind _sweepangle_2 (Variables|Default|GetSweepAngle))
  (bind _grabsphere (Variables|Default|GetGrabSphere))
  (bind _throwdistance (Variables|Default|GetThrowDistance))
  (bind _rotatingmovement (Variables|Default|GetRotatingMovement))
  (bind _transformcomponent (Variables|/Script/Engine.PlayerCameraManager|GetTransformComponent _returnvalue))
  (bind _returnvalue_2 (Transformation|GetWorldLocation _transformcomponent))
  (bind _returnvalue_3 (Math|Vector|GetForwardVector _transformcomponent))
  (bind _returnvalue_4 (* _returnvalue_3 _throwdistance))
  (bind _returnvalue_5 (* _returnvalue_3 _throwdistance))
  (Variables|Default|SetStartPoint (Transformation|GetWorldLocation (Variables|Default|GetRotationAxis)))
  (Components|Activation|SetActive _rotatingmovement true true)
  (Variables|/Script/Engine.RotatingMovementComponent|SetPivotTranslation _rotatingmovement (Variables|/Script/Engine.SceneComponent|GetRelativeLocation (Variables|Default|GetRotationAxis)))
  (Utilities|Casting|CastToLeftHand (Variables|Default|GetHand)
    (:then
      (Variables|/Script/Engine.RotatingMovementComponent|SetRotationRate _rotatingmovement _rotationspeed)
      (Variables|Default|SetCalibrationPoint (+ (/ _returnvalue_4 2.0) _returnvalue_2))
      (Variables|Default|SetTargetPoint1 (+ _returnvalue_4 _returnvalue_2))
      (Variables|Default|SetTargetPoint2 (+ (* (Math|Vector|RotateVector _returnvalue_3 (* _sweepangle 0.5)) (Variables|Default|GetThrowDistance)) _returnvalue_2))
      (Variables|Default|SetTargetPoint3 (+ (* (Math|Vector|RotateVector _returnvalue_3 _sweepangle) (Variables|Default|GetThrowDistance)) _returnvalue_2)))
    (:CastFailed
      (Variables|/Script/Engine.RotatingMovementComponent|SetRotationRate _rotatingmovement (* _rotationspeed -1))
      (Variables|Default|SetCalibrationPoint (+ _returnvalue_2 (/ _returnvalue_5 2.0)))
      (Variables|Default|SetTargetPoint1 (+ _returnvalue_2 _returnvalue_5))
      (Variables|Default|SetTargetPoint2 (+ _returnvalue_2 (* (Math|Vector|RotateVector _returnvalue_3 (* _sweepangle_2 -0.5)) (Variables|Default|GetThrowDistance))))
      (Variables|Default|SetTargetPoint3 (+ _returnvalue_2 (* (Math|Vector|RotateVector _returnvalue_3 (* _sweepangle_2 -1)) (Variables|Default|GetThrowDistance))))))
  (bind _returnvalue_6 (Effects|SpawnEmitterAttached "/Game/Materials/BoomerangRibbon.BoomerangRibbon" (Variables|Default|GetRotationAxis) "None"))
  (Variables|Default|SetTrail _returnvalue_6)
  (Collision|SetCollisionEnabled _grabsphere "QueryOnly")
  (Rendering|SetVisibility _grabsphere true false)
  (CallFunction|Fly)
  (Variables|Default|SetThrowState "NewEnumerator2"))

(event Custom|Fly
  (bind _returnvalue (Transformation|GetActorRotation))
  (bind _overlappingcomponents (Variables|Default|GetOverlappingComponents))
  (bind _hitbox2 (Variables|Default|GetHitbox2))
  (bind _flightpath (Variables|Default|GetFlightPath))
  (bind _flightpath_2 (Variables|Default|GetFlightPath))
  (bind _grabsphere (Variables|Default|GetGrabSphere))
  (bind _grabsphere_2 (Variables|Default|GetGrabSphere))
  (bind _inoverlappingcomponents (Class|PrimitiveComponent|GetOverlappingComponents _hitbox2))
  (bind (_roll _pitch _yaw) (Math|Rotator|BreakRotator _returnvalue))
  (bind _output_get (Variables|Default|SetStartPitch (.Pitch (Math|Rotator|BreakRotator (Transformation|GetActorRotation)))))
  (if (< _output_get 0.0)
    (Variables|Default|SetEndPitch 9e+01)
    (else
      (Variables|Default|SetEndPitch -9e+01)))
  (Spline|ClearSplinePoints _flightpath true)
  (for (_array_element _array_index) (Utilities|Array|MakeArray (Variables|Default|GetStartPoint) (Variables|Default|GetCalibrationPoint) (Variables|Default|GetTargetPoint1) (Variables|Default|GetTargetPoint2) (Variables|Default|GetTargetPoint3) (Variables|Default|GetStartPoint))
    (Spline|AddSplinePoint _flightpath _array_element "Local" true)
    (Spline|SetSplinePointType _flightpath _array_index "Curve" true))
  (bind (_direction _distancealongspline _rotation) (Timeline|Flight PlayFromStart)
    (:Update
      (if (Utilities|Enum|NotEqual(Enum) (Variables|Default|GetThrowState) "NewEnumerator3")
        (Utilities|FlowControl|Sequence
          (:then_0
            (Transformation|SetActorLocation (- (Spline|GetLocationatDistanceAlongSpline _flightpath_2 (* _distancealongspline (Spline|GetSplineLength _flightpath_2)) "Local") (Variables|/Script/Engine.SceneComponent|GetRelativeLocation (Variables|Default|GetRotationAxis))) false false)
            (Utilities|Array|Clear _overlappingcomponents)
            (Utilities|Array|AppendArray _overlappingcomponents (Class|PrimitiveComponent|GetOverlappingComponents (Variables|Default|GetHitbox)))
            (Utilities|Array|AppendArray _overlappingcomponents _inoverlappingcomponents)
            (bind _array_element_2 (Utilities|Array|ForEachLoopwithBreak _inoverlappingcomponents :!label _label)
              (:LoopBody
                (if (Utilities|Enum|Equal(Enum) (Collision|GetCollisionObjectType _array_element_2) "ECC_WorldStatic")
                  (Variables|Default|SetThrowState "NewEnumerator3")
                  (CallFunction|Fall)
                  (Collision|SetCollisionEnabled _grabsphere "NoCollision")
                  (Rendering|SetVisibility _grabsphere false false)
                  (goto _label Break)))))
          (:then_1
            (Transformation|SetActorRotation (Math|Rotator|MakeRotator _roll (Math|Float|Lerp (Variables|Default|GetStartPitch) 9e+01 _rotation) _yaw))))
        (else
          (Timeline|Flight Stop))))
    (:Finished
      (Collision|SetCollisionEnabled _grabsphere_2 "NoCollision")
      (Rendering|SetVisibility _grabsphere_2 false false)
      (if (Utilities|Enum|NotEqual(Enum) (Variables|Default|GetThrowState) "NewEnumerator3")
        (CallFunction|Fall)))))

(event EventTick
  (params (DeltaSeconds :type Float%20%28single-precision%29))
  (bind _hitbox (Variables|Default|GetHitBox))
  (bind _hitbox_2 (Variables|Default|GetHitBox))
  (bind _overlappingactors (Variables|Default|GetOverlappingActors))
  (bind _returnvalue (Transformation|GetWorldLocation _hitbox_2))
  (if (not (Variables|Default|GetIsMenuIcon))
    (bind _returnvalue_2 (Physics|GetPhysicsLinearVelocity _hitbox "None"))
    (if (or (>= (.Y (Math|Vector|BreakVector (Math|Vector|UnrotateVector _returnvalue_2 (Transformation|GetWorldRotation _hitbox)))) 1e+02) (Utilities|Enum|NotEqual(Enum) (Variables|Default|GetThrowState) "NewEnumerator3"))
      (Variables|Default|SetSlashing true)
      (Variables|Default|SetThisDamage (Variables|Default|GetSlashDamage))
      (Variables|Default|SetDamageType "/Game/Blueprints/DamageTypes/Slash.Slash_C")
      (Utilities|Array|Clear _overlappingactors)
      (Utilities|Array|AppendArray _overlappingactors (Collision|GetOverlappingActors (Variables|Default|GetHitBox) 0 :!class /Script/Engine.PrimitiveComponent))
      (Utilities|Array|AppendArray _overlappingactors (Collision|GetOverlappingActors (Variables|Default|GetHitBox2) 0 :!class /Script/Engine.PrimitiveComponent))
      (for _array_element _overlappingactors
        (if (Utilities|DoesObjectImplementInterface _array_element "/Game/Blueprints/Interfaces/Damageable.Damageable_C")
          (Game|Damage|ApplyPointDamage _array_element (Variables|Default|GetThisDamage) (- (Transformation|GetActorLocation _array_element) _returnvalue) (Collision|MakeHitResult false false 0.0 0.0 _returnvalue _returnvalue (- (Transformation|GetActorLocation _array_element) _returnvalue) (- (Transformation|GetActorLocation _array_element) _returnvalue) 0 _array_element) 0 self (Variables|Default|GetDamageType))))
      (else
        (Variables|Default|SetSlashing false)))))

(event EventBeginPlay
  (Collision|SetCollisionEnabled (Variables|Default|GetGrabSphere) "NoCollision"))

(event EventAttachtoMenu
  (params (Angle :type Rotator :default "0, 0, 0") (Orientation :type Rotator :default "0, 0, 0") (Position :type Vector :default "0, 0, 0") (Origin :type Scene%20Component%20Object%20Reference))
  (Variables|Default|SetIsMenuIcon true)
  (Physics|SetSimulatePhysics (Variables|Default|GetOrigin) false)
  (Transformation|AttachComponentToComponent Origin "None" "SnapToTarget" "SnapToTarget" "SnapToTarget" true)
  (Transformation|SetActorScale3D "0.100000,0.100000,0.100000")
  (Transformation|SetActorRelativeRotation Angle)
  (Transformation|AddActorLocalOffset Position false false)
  (Transformation|AddActorLocalRotation Orientation false false)
  (Transformation|AddActorLocalOffset (* (Variables|/Script/Engine.SceneComponent|GetRelativeLocation (Variables|Default|GetMiddle)) (Transformation|GetActorScale3D) "-1.000000,-1.000000,-1.000000") false false))

(event EventPickup
  (params (AttachTo :type Skeletal%20Mesh%20Component%20Object%20Reference) (Socket :type Name :default "None"))
  (bind _returnvalue (Game|GetPlayerCameraManager 0))
  (bind _returnvalue_2 (Components|GetOwner AttachTo))
  (bind _origin (Variables|Default|GetOrigin))
  (bind _gripthresh (Variables|Default|GetGripThresh))
  (bind _righthandgrip (Variables|Default|GetRightHandGrip))
  (bind _returnvalue_3 (Transformation|GetAttachParent _origin))
  (bind _transformcomponent (Variables|/Script/Engine.PlayerCameraManager|GetTransformComponent _returnvalue))
  (bind _returnvalue_4 (Components|GetOwner _returnvalue_3))
  (if (not (Variables|Default|GetIsMenuIcon))
    (CallFunction|Reset)
    (Utilities|FlowControl|Sequence
      (:then_0
        (if (and (!= _returnvalue_3 0) (!= _returnvalue_3 _returnvalue_2))
          (Actor|DestroyActor (Variables|Default|GetReticule))
          (Variables|Default|SetReticule 0)
          (bind _asleft_hand (Utilities|Casting|CastToLeftHand _returnvalue_4)
            (:then
              (Variables|/Game/Blueprints/Player/Hands/LeftHand.LeftHand_C|SetAttachedActor _asleft_hand 0))
            (:CastFailed
              (bind _asright_hand (Utilities|Casting|CastToRightHand _returnvalue_4))
              (Variables|/Game/Blueprints/Player/Hands/RightHand.RightHand_C|SetAttachedActor _asright_hand 0)))))
      (:then_1
        (Transformation|AttachComponentToComponent (Variables|Default|GetOrigin) AttachTo Socket "SnapToTarget" "SnapToTarget" "KeepWorld" true)
        (bind _output_get (Variables|Default|SetHand _returnvalue_2))
        (bind _asleft_hand_2 (Utilities|Casting|CastToLeftHand _output_get)
          (:then
            (Variables|/Game/Blueprints/Player/Hands/LeftHand.LeftHand_C|SetMaxGrip _asleft_hand_2 _gripthresh))
          (:CastFailed
            (bind _asright_hand_2 (Utilities|Casting|CastToRightHand _output_get))
            (Variables|/Game/Blueprints/Player/Hands/RightHand.RightHand_C|SetMaxGrip _asright_hand_2 _gripthresh)
            (Transformation|AddActorLocalRotation (Variables|/Script/Engine.SceneComponent|GetRelativeRotation _righthandgrip) false false)
            (Transformation|AddActorLocalOffset (* (Variables|/Script/Engine.SceneComponent|GetRelativeLocation _righthandgrip) (Transformation|GetWorldScale _righthandgrip) "1.000000,-1.000000,-1.000000") false false)))
        (bind _returnvalue_5 (Game|SpawnActorfromClass "/Game/Blueprints/Misc/Target.Target_C" (Math|Transform|MakeTransform (+ (* (Math|Vector|GetForwardVector _transformcomponent) (Variables|Default|GetThrowDistance)) (Transformation|GetWorldLocation _transformcomponent))) "Undefined" 0 0))
        (bind _output_get_2 (Variables|Default|SetReticule _returnvalue_5))
        (Transformation|AttachComponentToComponent _output_get_2 _transformcomponent "None" "KeepWorld" "SnapToTarget" "KeepWorld" true)))))

(event EventDrop
  (params (Dropper :type Actor%20Object%20Reference))
  (bind _category (Variables|Default|GetCategory))
  (Actor|DestroyActor (Variables|Default|GetReticule))
  (Variables|Default|SetReticule 0)
  (Transformation|DetachFromActor "KeepWorld" "KeepWorld" "KeepWorld")
  (if (Variables|Default|GetSlashing)
    (CallFunction|Throw)
    (else
      (Variables|Default|SetHand 0)
      (Physics|SetSimulatePhysics (Variables|Default|GetOrigin) true)
      (bind _array_element (Utilities|Array|ForEachLoopwithBreak (Collision|GetOverlappingActors "/Game/Blueprints/Player/LowerBackWeaponSpawn.LowerBackWeaponSpawn_C" :!class /Script/Engine.Actor))
        (:LoopBody
          (Utilities|Casting|CastToLowerBackWeaponSpawn _array_element)
          (bind _asvrcharacter (Utilities|Casting|CastToVRCharacter (Game|Player|GetPlayerPawn 0)))
          (bind _inventory (Default|GetInventoryCategory _asvrcharacter (Variables|Default|GetCategory)))
          (bind _index (Utilities|FlowControl|ForLoopwithBreak 0 (Utilities|Array|LastIndex _inventory) :!label _label)
            (:LoopBody
              (bind _placed (Default|SetInventoryCategory _asvrcharacter _category (Utilities|GetClass self) _index))
              (if _placed
                (Default|SetEquippedCategory _asvrcharacter _category _index)
                (Actor|DestroyActor)
                (goto _label Break)))
            (:Completed
              (bind _asmenu_base (Utilities|Casting|CastToMenuBase (Variables|/Game/Blueprints/Player/VRCharacter.VRCharacter_C|GetMenu _asvrcharacter)))
              (Variables|/Game/Blueprints/UI_Elements/Menu/MenuBase.MenuBase_C|SetCurrentDraw _asmenu_base "NewEnumerator2"))))))))

(fn ConstructionScript)

(fn HandleOverlaps)

(fn Fall
  (Variables|Default|SetThrowState "NewEnumerator3")
  (Variables|Default|SetHand 0)
  (Physics|SetSimulatePhysics (Variables|Default|GetOrigin) true)
  (Components|Activation|SetActive (Variables|Default|GetRotatingMovement) false true)
  (Components|DestroyComponent (Variables|Default|GetTrail))
  (Variables|Default|SetTrail 0))

(fn Reset
  (bind _grabsphere (Variables|Default|GetGrabSphere))
  (Utilities|FlowControl|Sequence
    (:then_0
      (if (!= (Variables|Default|GetTrail) 0)
        (Components|DestroyComponent (Variables|Default|GetTrail))
        (Variables|Default|SetTrail 0)))
    (:then_1
      (Collision|SetCollisionEnabled _grabsphere "NoCollision")
      (Rendering|SetVisibility _grabsphere false false)
      (Components|Activation|SetActive (Variables|Default|GetRotatingMovement) false true)
      (Physics|SetSimulatePhysics (Variables|Default|GetOrigin) false)
      (Variables|Default|SetThrowState "NewEnumerator3"))))