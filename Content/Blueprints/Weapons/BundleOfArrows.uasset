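; Grabbable VR arrow bundle that converts into arrow inventory when released over the player's back.
; Pickup releases it from any previous hand, snaps it to the new socket and sets that hand's grip limit.
; Drop restores physics and, over a BackWeaponSpawn, adds seven arrows, tries to equip them, updates the menu and destroys itself, even if adding fails.
; IgnorePlayer disables movement collision with the player, attached actors and arrows.
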(event EventDrop
  (params (Dropper :type Actor%20Object%20Reference))
  (bind _category (Variables|Default|GetCategory))
  (Physics|SetSimulatePhysics (Variables|Default|GetOrigin) true)
  (Transformation|DetachFromActor "KeepWorld" "KeepWorld" "KeepWorld")
  (bind _array_element (Utilities|Array|ForEachLoopwithBreak (Collision|GetOverlappingActors "/Game/Blueprints/Player/BackWeaponSpawn.BackWeaponSpawn_C" :!class /Script/Engine.Actor))
    (:LoopBody
      (Utilities|Casting|CastToBackWeaponSpawn _array_element)
      (bind _asvrcharacter (Utilities|Casting|CastToVRCharacter (Game|Player|GetPlayerPawn 0)))
      (bind _inventory (Default|GetInventoryCategory _asvrcharacter (Variables|Default|GetCategory)))
      (bind _addednew (Default|AddItem _asvrcharacter "/Game/Blueprints/Weapons/Arrow.Arrow_C" 7))
      (if _addednew
        (bind _index (Utilities|FlowControl|ForLoopwithBreak 0 (Utilities|Array|LastIndex _inventory) :!label _label)
          (:LoopBody
            (bind _placed (Default|SetInventoryCategory _asvrcharacter _category "/Game/Blueprints/Weapons/Arrow.Arrow_C" _index))
            (if _placed
              (Default|SetEquippedCategory _asvrcharacter _category _index)
              (goto _label Break)))
          (:Completed
            (Utilities|FlowControl|Sequence :!label _label_2
              (:then_0
                (bind _asmenu_base (Utilities|Casting|CastToMenuBase (Variables|/Game/Blueprints/Player/VRCharacter.VRCharacter_C|GetMenu _asvrcharacter)))
                (Variables|/Game/Blueprints/UI_Elements/Menu/MenuBase.MenuBase_C|SetCurrentDraw _asmenu_base "NewEnumerator2"))
              (:then_1
                (Actor|DestroyActor)))))
        (else
          (goto _label_2))))))

(event EventPickup
  (params (AttachTo :type Skeletal%20Mesh%20Component%20Object%20Reference) (Socket :type Name :default "None"))
  (bind _returnvalue (Components|GetOwner AttachTo))
  (bind _origin (Variables|Default|GetOrigin))
  (bind _gripthresh (Variables|Default|GetGripThresh))
  (bind _returnvalue_2 (Transformation|GetAttachParent _origin))
  (bind _returnvalue_3 (Components|GetOwner _returnvalue_2))
  (if (not (Variables|Default|GetIsMenuIcon))
    (Physics|SetSimulatePhysics (Variables|Default|GetOrigin) false)
    (Utilities|FlowControl|Sequence
      (:then_0
        (if (and (!= _returnvalue_2 0) (!= _returnvalue_2 _returnvalue))
          (bind _asleft_hand (Utilities|Casting|CastToLeftHand _returnvalue_3)
            (:then
              (Variables|/Game/Blueprints/Player/Hands/LeftHand.LeftHand_C|SetAttachedActor _asleft_hand 0))
            (:CastFailed
              (bind _asright_hand (Utilities|Casting|CastToRightHand _returnvalue_3))
              (Variables|/Game/Blueprints/Player/Hands/RightHand.RightHand_C|SetAttachedActor _asright_hand 0)))))
      (:then_1
        (Transformation|AttachComponentToComponent (Variables|Default|GetOrigin) AttachTo Socket "SnapToTarget" "SnapToTarget" "KeepWorld" true)
        (bind _asleft_hand_2 (Utilities|Casting|CastToLeftHand _returnvalue)
          (:then
            (Variables|/Game/Blueprints/Player/Hands/LeftHand.LeftHand_C|SetMaxGrip _asleft_hand_2 _gripthresh))
          (:CastFailed
            (bind _asright_hand_2 (Utilities|Casting|CastToRightHand _returnvalue))
            (Variables|/Game/Blueprints/Player/Hands/RightHand.RightHand_C|SetMaxGrip _asright_hand_2 _gripthresh)))))))

(fn ConstructionScript)

(fn IgnorePlayer
  (bind _returnvalue (Game|Player|GetPlayerPawn 0))
  (bind _origin (Variables|Default|GetOrigin))
  (Collision|IgnoreActorwhenMoving _origin _returnvalue true)
  (for _array_element (Actor|GetAttachedActors _returnvalue)
    (Collision|IgnoreActorwhenMoving _origin _array_element true))
  (for _array_element_2 (Actor|GetAllChildActors _returnvalue true)
    (for _array_element_3 (Actor|GetAttachedActors _array_element_2)
      (Collision|IgnoreActorwhenMoving _origin _array_element_3 true)))
  (bind _outactors (Actor|GetAllActorswithInterface "/Game/Blueprints/Interfaces/Arrow.Arrow_C"))
  (for _array_element_4 _outactors
    (Collision|IgnoreActorwhenMoving _origin _array_element_4 true)))