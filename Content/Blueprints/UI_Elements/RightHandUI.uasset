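; Right-hand VR UI actor that displays an item model and quantity for money, bombs or arrows, based on what the player holds.
; Each tick in the Static state, GetItemAndState scans both hands' attached actors via Bow, Arrow and Bomb interfaces, defaulting to green rupees.
; Changes in item, mode or count trigger Clear, which destroys attached actors, then Draw, which spawns a collision-free model and updates the count text.
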(event EventTick
  (params (DeltaSeconds :type Float%20%28single-precision%29))
  (bind _returnvalue (Game|Player|GetPlayerPawn 0))
  (switch Utilities|FlowControl|Switch|SwitchonRightHandUIState (Variables|Default|GetDrawState)
    (:NewEnumerator3
      (bind _arrayelement (Utilities|Array|ReverseforEachLoop (Actor|GetAttachedActors))
        (:LoopBody
          (Actor|DestroyActor _arrayelement))
        (:Completed
          (Variables|Default|SetDrawState "NewEnumerator4"))))
    (:NewEnumerator4
      (Utilities|FlowControl|Sequence
        (:then_0
          (switch Utilities|FlowControl|Switch|SwitchonUIDrawStates (Variables|Default|GetUIState)
            (:NewEnumerator0
              (bind _returnvalue_2 (Game|SpawnActorfromClass (Variables|Default|GetDrawItem) (Math|Transform|MakeTransform "0, 0, 0") "Undefined" 0 0))
              (Class|Icon|AttachtoMenu(Message) _returnvalue_2 "0, 0, 0" "0.000000,0,0.000000" "0, 0, 0" (Variables|Default|GetBase))
              (Collision|SetActorEnableCollision _returnvalue_2 false)
              (bind _asvrcharacter (Utilities|Casting|CastToVRCharacter (Game|Player|GetPlayerPawn 0)))
              (bind _resultstat (Default|GetStat _asvrcharacter "NewEnumerator3"))
              (Variables|Default|SetCurrentQuantity _resultstat))
            (:NewEnumerator1
              (bind _asvrcharacter_2 (Utilities|Casting|CastToVRCharacter _returnvalue))
              (bind _quantity (Default|ItemQuantity _asvrcharacter_2 (Variables|Default|GetDrawItem)))
              (if (< _quantity 0)
                (Variables|Default|SetCurrentQuantity 0)
                (else
                  (Variables|Default|SetCurrentQuantity _quantity)
                  (bind _returnvalue_3 (Game|SpawnActorfromClass (Variables|Default|GetDrawItem) (Math|Transform|MakeTransform "0, 0, 0") "Undefined" 0 0))
                  (Class|Icon|AttachtoMenu(Message) _returnvalue_3 "0, 0, 0" "0.000000,0,0.000000" "0, 0, 0" (Variables|Default|GetBase))
                  (Collision|SetActorEnableCollision _returnvalue_3 false))))
            (:NewEnumerator2
              (bind _asvrcharacter_3 (Utilities|Casting|CastToVRCharacter _returnvalue))
              (bind _quantity_2 (Default|ItemQuantity _asvrcharacter_3 (Variables|Default|GetDrawItem)))
              (if (< _quantity_2 0)
                (Variables|Default|SetCurrentQuantity 0)
                (else
                  (Variables|Default|SetCurrentQuantity _quantity_2)
                  (bind _returnvalue_4 (Game|SpawnActorfromClass (Variables|Default|GetDrawItem) (Math|Transform|MakeTransform "0, 0, 0") "Undefined" 0 0))
                  (Class|Icon|AttachtoMenu(Message) _returnvalue_4 "0, 0, 0" "0.000000,0,0.000000" "0, 0, 0" (Variables|Default|GetBase))
                  (Collision|SetActorEnableCollision _returnvalue_4 false))))))
        (:then_1
          (Rendering|Components|TextRender|SetText (Variables|Default|GetQuantity) (Utilities|Text|FormatText "x{quantity}" (Variables|Default|GetCurrentQuantity)))
          (Variables|Default|SetDrawState "NewEnumerator5"))))
    (:NewEnumerator5
      (bind _asvrcharacter_4 (Utilities|Casting|CastToVRCharacter (Game|Player|GetPlayerPawn 0)))
      (bind (_newitem _newstate) (CallFunction|GetItemandState))
      (if (Utilities|Enum|NotEqual(Enum) _newstate (Variables|Default|GetUIState))
        (Variables|Default|SetDrawItem _newitem)
        (Variables|Default|SetUIState _newstate)
        (Variables|Default|SetDrawState "NewEnumerator3")
        (elif (!= _newitem (Variables|Default|GetDrawItem))
          (Variables|Default|SetDrawItem _newitem)
          (Variables|Default|SetDrawState "NewEnumerator3")
          (else
            (switch Utilities|FlowControl|Switch|SwitchonUIDrawStates _newstate
              (:NewEnumerator0
                (Variables|Default|SetDrawItem "/Game/Blueprints/Money/GreenRupee.GreenRupee_C")
                (bind _resultstat_2 (Default|GetStat _asvrcharacter_4 "NewEnumerator3"))
                (if (!= _resultstat_2 (Variables|Default|GetCurrentQuantity))
                  (Variables|Default|SetDrawState "NewEnumerator3")))
              (:NewEnumerator1
                (bind _quantity_3 (Default|ItemQuantity _asvrcharacter_4 _newitem :!label _label))
                (if (!= _quantity_3 (Variables|Default|GetCurrentQuantity))
                  (if (not (and (< _quantity_3 0) (== (Variables|Default|GetCurrentQuantity) 0)))
                    (Variables|Default|SetDrawState "NewEnumerator3"))))
              (:NewEnumerator2
                (goto _label)))))))))

(fn ConstructionScript)

(fn GetItemandState
  (bind _asvrcharacter (Utilities|Casting|CastToVRCharacter (Game|Player|GetPlayerPawn 0)))
  (for _array_element (Actor|GetAllChildActors _asvrcharacter true)
    (bind _asright_hand (Utilities|Casting|CastToRightHand _array_element)
      (:then
        (for _array_element_2 (Actor|GetAttachedActors _asright_hand)
          (if (Utilities|DoesObjectImplementInterface _array_element_2 "/Game/Blueprints/Interfaces/Bow.Bow_C")
            (LocalVariables|SetBowInHand true)
            (elif (Utilities|DoesObjectImplementInterface _array_element_2 "/Game/Blueprints/Interfaces/Arrow.Arrow_C")
              (LocalVariables|SetArrowInHand (Utilities|GetClass _array_element_2))
              (elif (Utilities|DoesObjectImplementInterface _array_element_2 "/Game/Blueprints/Interfaces/Bomb.Bomb_C")
                (LocalVariables|SetBombInHand (Utilities|GetClass _array_element_2)))))))
      (:CastFailed
        (bind _asleft_hand (Utilities|Casting|CastToLeftHand _array_element))
        (for _array_element_3 (Actor|GetAttachedActors _asleft_hand)
          (if (Utilities|DoesObjectImplementInterface _array_element_3 "/Game/Blueprints/Interfaces/Bow.Bow_C")
            (LocalVariables|SetBowInHand true)
            (elif (Utilities|DoesObjectImplementInterface _array_element_3 "/Game/Blueprints/Interfaces/Arrow.Arrow_C")
              (LocalVariables|SetArrowInHand (Utilities|GetClass _array_element_3))
              (elif (Utilities|DoesObjectImplementInterface _array_element_3 "/Game/Blueprints/Interfaces/Bomb.Bomb_C")
                (LocalVariables|SetBombInHand (Utilities|GetClass _array_element_3)))))))))
  (if (!= (LocalVariables|GetArrowInHand) 0)
    (return (LocalVariables|GetArrowInHand) "NewEnumerator2")
    (elif (LocalVariables|GetBowInHand)
      (bind _inventory (Default|GetInventoryCategory _asvrcharacter "NewEnumerator3"))
      (bind _equipped (Default|GetEquippedCategory _asvrcharacter "NewEnumerator3"))
      (return (Utilities|Array|Get(acopy) _inventory _equipped) "NewEnumerator2")
      (elif (!= (LocalVariables|GetBombInHand) 0)
        (return (LocalVariables|GetBombInHand) "NewEnumerator1")
        (else
          (return "/Game/Blueprints/Money/GreenRupee.GreenRupee_C" "NewEnumerator0"))))))