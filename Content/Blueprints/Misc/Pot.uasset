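; Breakable pot that drops an item when its Destructible component fractures.
; On BeginPlay, unless SpawnExclusive is set, PickItem makes a weighted random choice from the ItemRarity map to replace ItemToSpawn.
; The first fracture sets Broken to block repeat drops, spawns the item at the Middle component's transform, then destroys the pot after a short delay.
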(event OnComponentFracture(Destructible)
  (params (HitPoint :type Vector%20%28by%20ref%29 :default "0, 0, 0") (HitDirection :type Vector%20%28by%20ref%29 :default "0, 0, 0"))
  (if (not (Variables|Default|GetBroken))
    (Utilities|FlowControl|Sequence
      (:then_0
        (Variables|Default|SetBroken true)
        (Game|SpawnActorfromClass (Variables|Default|GetItemToSpawn) (Transformation|GetWorldTransform (Variables|Default|GetMiddle)) "Undefined" 0 0))
      (:then_1
        (Utilities|FlowControl|Delay 2.0)
        (Actor|DestroyActor)))))

(event EventBeginPlay
  (if (not (Variables|Default|GetSpawnExclusive))
    (bind _item (CallFunction|PickItem))
    (Variables|Default|SetItemToSpawn _item)))

(fn ConstructionScript)

(fn PickItem
  (bind _itemrarity (Variables|Default|GetItemRarity))
  (bind _values (Utilities|Map|Values (Variables|Default|GetItemRarity)))
  (for _array_element _values
    (LocalVariables|SetSum (+ _array_element (LocalVariables|GetSum))))
  (LocalVariables|SetRandomNumber (Math|Random|RandomInteger (LocalVariables|GetSum)))
  (bind _keys (Utilities|Map|Keys _itemrarity))
  (for _array_element_2 _keys
    (if (>= (+ (.Value (Utilities|Map|Find _itemrarity _array_element_2)) (LocalVariables|GetSumSoFar)) (LocalVariables|GetRandomNumber))
      (return _array_element_2)
      (else
        (LocalVariables|SetSumSoFar (+ (.Value (Utilities|Map|Find _itemrarity _array_element_2)) (LocalVariables|GetSumSoFar))))))
  (return 0))