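; Campfire actor that can be lit or put out and deals radial fire damage around its hitbox while lit.
; A looping timer calls Burn, which also fires immediately on hitbox overlap.
; Fire damage ignites it and Blunt damage extinguishes it, toggling particles, light and timer.
; The burn interval is shorter when ignited by damage than when lit at BeginPlay.
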(event OnComponentBeginOverlap(Hitbox)
  (params (OverlappedComponent :type Primitive%20Component%20Object%20Reference) (OtherActor :type Actor%20Object%20Reference) (OtherComp :type Primitive%20Component%20Object%20Reference) (OtherBodyIndex :type Integer) (bFromSweep :type Boolean) (SweepResult :type Hit%20Result%20Structure%20%28by%20ref%29))
  (if (Variables|Default|GetOn)
    (CallFunction|Burn)))

(event Game|Damage|EventAnyDamage
  (params (Damage :type Float%20%28single-precision%29) (DamageType :type Damage%20Type%20Object%20Reference) (InstigatedBy :type Controller%20Object%20Reference) (DamageCauser :type Actor%20Object%20Reference))
  (bind _returnvalue (Utilities|GetClass DamageType))
  (bind _particlesystem (Variables|Default|GetParticleSystem))
  (bind _pointlight (Variables|Default|GetPointLight))
  (if (== _returnvalue "/Game/Blueprints/DamageTypes/Fire.Fire_C")
    (if (not (Variables|Default|GetOn))
      (Components|Activation|Activate _particlesystem false)
      (Rendering|SetVisibility _pointlight true false)
      (Utilities|Time|SetTimerbyFunctionName 0 "Burn" 0.5 true)
      (Variables|Default|SetOn true))
    (elif (and (Variables|Default|GetOn) (== _returnvalue "/Game/Blueprints/DamageTypes/Blunt.Blunt_C"))
      (Components|Activation|Deactivate _particlesystem)
      (Rendering|SetVisibility _pointlight false false)
      (Utilities|Time|ClearTimerbyFunctionName 0 "Burn")
      (Variables|Default|SetOn false))))

(event EventBeginPlay
  (if (Variables|Default|GetOn)
    (Components|Activation|Activate (Variables|Default|GetParticleSystem) false)
    (Rendering|SetVisibility (Variables|Default|GetPointLight) true false)
    (Utilities|Time|SetTimerbyFunctionName 0 "Burn" 1.0 true)))

(fn ConstructionScript)

(fn Burn
  (Game|Damage|ApplyRadialDamage (Variables|Default|GetDamage) (Transformation|GetWorldLocation (Variables|Default|GetHitbox)) (Variables|Default|GetRadius) "/Game/Blueprints/DamageTypes/Fire.Fire_C" 0 self 0 true "ECC_Visibility"))