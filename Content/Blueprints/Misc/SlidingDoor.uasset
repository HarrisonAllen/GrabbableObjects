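; Sliding door actor that opens after it has been activated a set number of times.
; Each Activate call decrements TimesToActivate, and once it reaches zero or below, an Open timeline plays.
; The timeline's DistanceAlong track lerps the actor from its BeginPlay location to EndLocation, moving it without sweep.
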(event EventBeginPlay
  (Variables|Default|SetStartLocation (Transformation|GetActorLocation)))

(event EventActivate
  (bind _result (Math|Integer|DecrementInt (Variables|Default|GetTimesToActivate))
    (:%20%20
      (if (<= _result 0)
        (bind _distancealong (Timeline|Open Play)
          (:Update
            (Transformation|SetActorLocation (Math|Vector|Lerp(Vector) (Variables|Default|GetStartLocation) (Variables|Default|GetEndLocation) _distancealong) false false)))))))

(fn ConstructionScript)