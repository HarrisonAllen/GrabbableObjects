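; Damageable target dummy that displays health, hit type and damage taken on text components, then explodes at zero health and optionally respawns a copy.
; Recognized damage types subtract damage minus Defense.
; A cooldown blocks further hits until the delay ends and the damage causer stops overlapping Body, checked on Tick.
; Fire hits start a looping timer that applies Burn self-damage through the same damage path until its tick counter runs out.
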(event EventTick
  (params (DeltaSeconds :type Float%20%28single-precision%29))
  (Utilities|FlowControl|Sequence
    (:then_0
      (if (Variables|Actor|GetbCanBeDamaged)
        (Rendering|Components|TextRender|SetText (Variables|Default|GetHP) (Utilities|Text|ToText(Float) (Variables|Default|GetHealth) "HalfToEven"))))
    (:then_1
      (if (== (Variables|Default|GetFireTick) 0)
        (Utilities|Time|ClearTimerbyFunctionName 0 "Burn")
        (Variables|Default|SetFireTick -1)))
    (:then_2
      (if (and (Variables|Default|GetCooldown) (not (Collision|IsOverlappingActor (Variables|Default|GetBody) (Variables|Default|GetOverlap) :!class /Script/Engine.PrimitiveComponent)))
        (Variables|Default|SetCooldown false)
        (Variables|Actor|SetbCanBeDamaged true)
        (Variables|Default|SetOverlap 0)))))

(event EventBeginPlay
  (Variables|Default|SetHealth (Variables|Default|GetMaxHealth)))

(event Game|Damage|EventAnyDamage
  (params (Damage :type Float%20%28single-precision%29) (DamageType :type Damage%20Type%20Object%20Reference) (InstigatedBy :type Controller%20Object%20Reference) (DamageCauser :type Actor%20Object%20Reference))
  (bind _defense (Variables|Default|GetDefense))
  (bind _returnvalue (- Damage _defense))
  (bind _returnvalue_2 (Math|Float|Clamp(Float) _returnvalue 0.0 1e+04))
  (if (Variables|Actor|GetbCanBeDamaged)
    (Variables|Actor|SetbCanBeDamaged false)
    (Variables|Default|SetOverlap DamageCauser)
    (bind _hit (CallFunction|AnalyzeHit (Utilities|GetClass DamageType)))
    (if _hit
      (bind _output_get (Variables|Default|SetHealth (- (Variables|Default|GetHealth) _returnvalue_2)))
      (if (<= _output_get 0.0)
        (Gameplay|Die)
        (else
          (Rendering|Components|TextRender|SetText (Variables|Default|GetDamage) (Utilities|Text|ToText(Integer) (Math|Float|Floor (* -1 _returnvalue_2))))
          (if (== (Variables|Default|GetOverlap) self)
            (Utilities|FlowControl|Delay (/ (Variables|Default|GetCooldownTime) 2.0))
            (Variables|Default|SetOverlap 0)
            (else
              (Utilities|FlowControl|Delay (Variables|Default|GetCooldownTime))))
          (Variables|Default|SetCooldown true)
          (Rendering|Components|TextRender|SetText (Variables|Default|GetDamage) (Utilities|Text|MakeLiteralText "")))))))

(fn ConstructionScript)

(fn AnalyzeHit
  (params (HitType :type Object%20Class%20Reference))
  (bind _hp (Variables|Default|GetHP))
  (Utilities|FlowControl|Sequence
    (:then_0
      (if (== HitType "/Game/Blueprints/DamageTypes/Slash.Slash_C")
        (Rendering|Components|TextRender|SetText _hp (Utilities|Text|MakeLiteralText "Slash"))
        (return true)))
    (:then_1
      (if (== HitType "/Game/Blueprints/DamageTypes/Pierce.Pierce_C")
        (Rendering|Components|TextRender|SetText _hp (Utilities|Text|MakeLiteralText "Pierce"))
        (return true)))
    (:then_2
      (if (== HitType "/Game/Blueprints/DamageTypes/Blunt.Blunt_C")
        (Rendering|Components|TextRender|SetText _hp (Utilities|Text|MakeLiteralText "Blunt"))
        (return true)))
    (:then_3
      (if (== HitType "/Game/Blueprints/DamageTypes/BadSlash.BadSlash_C")
        (Rendering|Components|TextRender|SetText _hp (Utilities|Text|MakeLiteralText "Bad Slash"))
        (return true)))
    (:then_4
      (if (== HitType "/Game/Blueprints/DamageTypes/Explosion.Explosion_C")
        (Rendering|Components|TextRender|SetText _hp (Utilities|Text|MakeLiteralText "Explosion"))
        (return true)))
    (:then_5
      (if (== HitType "/Game/Blueprints/DamageTypes/Fire.Fire_C")
        (Rendering|Components|TextRender|SetText _hp (Utilities|Text|MakeLiteralText "Fire"))
        (Variables|Default|SetOnFire? true)
        (Variables|Default|SetFireTick 6)
        (Utilities|Time|SetTimerbyFunctionName 0 "Burn" 1.0 true)
        (return true)))
    (:then_6
      (if (== HitType "/Game/Blueprints/DamageTypes/Burn.Burn_C")
        (Rendering|Components|TextRender|SetText _hp (Utilities|Text|MakeLiteralText "Burn"))
        (return true)))
    (:then_7
      (return false))))

(fn Burn
  (Game|Damage|ApplyDamage self 5.0 0 self "/Game/Blueprints/DamageTypes/Burn.Burn_C")
  (Math|Integer|DecrementInt (Variables|Default|GetFireTick)))