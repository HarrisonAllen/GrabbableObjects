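; VR back holster that follows the camera's position and yaw, spawning an inventory weapon into the hand that grabs it.
; Pickup takes the item selected in the open menu, or smart-grabs a category from the other hand's sword or bow, else by grabbing hand.
; The spawned item attaches through PickupMessage and its slot is cleared, except bow-companion arrows, which decrement until empty.
; An open menu showing that category is redrawn.
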(event EventTick
  (params (DeltaSeconds :type Float%20%28single-precision%29))
  (bind _returnvalue (Game|GetPlayerCameraManager 0))
  (bind _returnvalue_2 (Transformation|GetActorTransform _returnvalue))
  (bind (_location _rotation) (Math|Transform|BreakTransform _returnvalue_2))
  ;[1 1 1] Always follow the player and attach to their back, but always stay vertical
  (Transformation|SetWorldLocationAndRotation (Variables|Default|GetDefaultSceneRoot) _location (Math|Rotator|MakeRotator 0.0 0.0 (.Yaw (Math|Rotator|BreakRotator _rotation))) false true)
  (Transformation|AddActorLocalOffset "-30.000000,0.000000,0.000000" false false)
  (Class|Actor|AddActorWorldRotation "0,90.000000, 0"))

(event EventPickup
  (params (AttachTo :type Skeletal%20Mesh%20Component%20Object%20Reference) (Socket :type Name :default "None"))
  (bind _asvrcharacter (Utilities|Casting|CastToVRCharacter (Game|Player|GetPlayerPawn 0)))
  (bind _asmenu_base (Utilities|Casting|CastToMenuBase (Variables|/Game/Blueprints/Player/VRCharacter.VRCharacter_C|GetMenu _asvrcharacter))
    (:then
      (Variables|Default|SetMenu? true))
    (:CastFailed
      (Variables|Default|SetMenu? false)))
  (Utilities|FlowControl|Sequence
    (:then_0
      ;[1 1 1] Checks which hand is grabbing -> this hand. Other hand is, well, the other hand.
      (bind _array_element (Utilities|Array|ForEachLoopwithBreak (Actor|GetAllChildActors _asvrcharacter true))
        (:LoopBody
          (if (== _array_element (Components|GetOwner AttachTo))
            (Variables|Default|SetThisHand _array_element)
            (else
              (bind _asleft_hand (Utilities|Casting|CastToLeftHand _array_element)
                (:then
                  (Variables|Default|SetOtherHand _asleft_hand))
                (:CastFailed
                  (bind _asright_hand (Utilities|Casting|CastToRightHand _array_element))
                  (Variables|Default|SetOtherHand _asright_hand))))))))
    (:then_1
      ;[1 1 1] Check for bows or swords in hand. This will enable a smart grab system, where we pull out a shield if we've already got a sword, and an arrow if we've already got a bow
      (bind _array_element_2 (Utilities|Array|ForEachLoopwithBreak (Actor|GetAttachedActors (Variables|Default|GetOtherHand)) :!label _label)
        (:LoopBody
          (if (Utilities|DoesObjectImplementInterface _array_element_2 "/Game/Blueprints/Interfaces/Sword.Sword_C")
            (Variables|Default|SetSwordInHand true)
            (goto _label Break)
            (elif (Utilities|DoesObjectImplementInterface _array_element_2 "/Game/Blueprints/Interfaces/Bow.Bow_C")
              (Variables|Default|SetBowInHand true)
              (goto _label Break))))))
    (:then_2
      ;[1 1 1] Decide what to pull out. If the player is hovering over an item in the menu, choose that. Otherwise, pull out a smart grab.
      (if (Variables|Default|GetMenu?)
        (if (Math|Boolean|ANDBoolean (Utilities|Enum|NotEqual(Enum) (Variables|/Game/Blueprints/UI_Elements/Menu/MenuBase.MenuBase_C|GetCurrentMenu _asmenu_base) "NewEnumerator7") (Utilities|Enum|NotEqual(Enum) (Variables|/Game/Blueprints/UI_Elements/Menu/MenuBase.MenuBase_C|GetCurrentMenu _asmenu_base) "NewEnumerator7") (Utilities|Enum|NotEqual(Enum) (Variables|/Game/Blueprints/UI_Elements/Menu/MenuBase.MenuBase_C|GetCurrentMenu _asmenu_base) "NewEnumerator9") (Utilities|Enum|NotEqual(Enum) (Variables|/Game/Blueprints/UI_Elements/Menu/MenuBase.MenuBase_C|GetCurrentMenu _asmenu_base) "NewEnumerator6") (Utilities|Enum|NotEqual(Enum) (Variables|/Game/Blueprints/UI_Elements/Menu/MenuBase.MenuBase_C|GetCurrentMenu _asmenu_base) "NewEnumerator8"))
          (bind _category (Default|MenutoCategory _asmenu_base (Variables|/Game/Blueprints/UI_Elements/Menu/MenuBase.MenuBase_C|GetCurrentMenu _asmenu_base)))
          (Variables|Default|SetCategory _category)
          (if (> (Variables|/Game/Blueprints/UI_Elements/Menu/MenuBase.MenuBase_C|GetMenuIndex _asmenu_base) 0)
            (bind _output_get (Variables|Default|SetIndex (- (Variables|/Game/Blueprints/UI_Elements/Menu/MenuBase.MenuBase_C|GetMenuIndex _asmenu_base) 1)))
            (Default|SetEquippedCategory _asvrcharacter (Variables|Default|GetCategory) _output_get)
            (else
              (bind _equipped (Default|GetEquippedCategory _asvrcharacter (Variables|Default|GetCategory) :!label _label_2))
              (Variables|Default|SetIndex _equipped)))
          (else
            (Utilities|FlowControl|Sequence :!label _label_3
              (:then_0
                (if (Variables|Default|GetSwordInHand)
                  (Variables|Default|SetCategory "NewEnumerator1")
                  (elif (Variables|Default|GetBowInHand)
                    (Variables|Default|SetCategory "NewEnumerator3")
                    (else
                      (Utilities|Casting|CastToLeftHand (Variables|Default|GetThisHand)
                        (:then
                          (Variables|Default|SetCategory "NewEnumerator2"))
                        (:CastFailed
                          (Variables|Default|SetCategory "NewEnumerator0")))))))
              (:then_1
                (goto _label_2)))))
        (else
          (goto _label_3))))
    (:then_3
      ;[1 1 1] Pull the weapon out of the bag and give it to the hand that called it.
      (bind _inventory (Default|GetInventoryCategory _asvrcharacter (Variables|Default|GetCategory)))
      (if (!= (Utilities|Array|Get(acopy) _inventory (Variables|Default|GetIndex)) 0)
        (if (Utilities|Enum|Equal(Enum) (Variables|Default|GetCategory) "NewEnumerator3")
          (bind (_empty _couldremove) (Default|RemoveItem _asvrcharacter (Utilities|Array|Get(acopy) _inventory (Variables|Default|GetIndex)) 1))
          (if _couldremove
            (bind _returnvalue (Game|SpawnActorfromClass (Utilities|Array|Get(acopy) _inventory (Variables|Default|GetIndex)) (Transformation|GetActorTransform) "Undefined" 0 0 :!label _label_4))
            (bind _asright_hand_2 (Utilities|Casting|CastToRightHand (Variables|Default|GetThisHand))
              (:then
                (bind _output_get_2 (Variables|/Game/Blueprints/Player/Hands/RightHand.RightHand_C|SetAttachedActor _asright_hand_2 _returnvalue))
                (Class|GrabbableInterface|Pickup(Message) _output_get_2 AttachTo Socket))
              (:CastFailed
                (bind _asleft_hand_2 (Utilities|Casting|CastToLeftHand (Variables|Default|GetThisHand)))
                (bind _output_get_3 (Variables|/Game/Blueprints/Player/Hands/LeftHand.LeftHand_C|SetAttachedActor _asleft_hand_2 _returnvalue))
                (Class|GrabbableInterface|Pickup(Message) _output_get_3 AttachTo Socket)))
            (if (or _empty (not (Utilities|Enum|Equal(Enum) (Variables|Default|GetCategory) "NewEnumerator3")))
              (Default|ClearInventoryCategory _asvrcharacter (Variables|Default|GetCategory) (Variables|Default|GetIndex)))
            (Variables|Default|SetBowInHand false)
            (Variables|Default|SetSwordInHand false))
          (else
            (goto _label_4)))))
    (:then_4
      ;[1 1 1] Update the menu if we've made any changes to the sub menu
      (if (Variables|Default|GetMenu?)
        (bind _category_2 (Default|MenutoCategory _asmenu_base (Variables|/Game/Blueprints/UI_Elements/Menu/MenuBase.MenuBase_C|GetCurrentMenu _asmenu_base)))
        (if (Utilities|Enum|Equal(Enum) _category_2 (Variables|Default|GetCategory))
          (Variables|/Game/Blueprints/UI_Elements/Menu/MenuBase.MenuBase_C|SetCurrentDraw _asmenu_base "NewEnumerator2"))))))

(fn ConstructionScript)