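; VR player character that holds the player's inventory, equipped slots, item quantities and health/money stats, with accessor functions for each.
; BeginPlay hides the controllers and spawns back weapon volumes, an item bag, an optional grappling hook and a right-hand UI.
; While no menu is open, Tick turns joystick push-then-release into a directional menu on the left hand, with left/right choices depending on held bow or arrow.
; The special-right button opens a default menu.
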(event EventBeginPlay
  (bind _returnvalue (Math|Transform|MakeTransform "0, 0, 0"))
  (Utilities|FlowControl|Sequence
    (:then_0
      (Class|HeadMountedDisplayFunctionLibrary|SetTrackingOrigin "Floor")
      (Rendering|SetVisibility (Variables|Default|GetLeftController) false true)
      (Rendering|SetVisibility (Variables|Default|GetRightController) false true))
    (:then_1
      (bind _returnvalue_2 (Game|SpawnActorfromClass "/Game/Blueprints/Player/BackWeaponSpawn.BackWeaponSpawn_C" _returnvalue "Undefined" 0 0))
      (Variables|Default|SetBackSpawnVolume _returnvalue_2))
    (:then_2
      (bind _returnvalue_3 (Game|SpawnActorfromClass "/Game/Blueprints/Player/LowerBackWeaponSpawn.LowerBackWeaponSpawn_C" _returnvalue "Undefined" 0 0))
      (Variables|Default|SetLowerBackSpawnVolume _returnvalue_3))
    (:then_3
      (if (Variables|Default|GetHasGrapplingHook)
        (Game|SpawnActorfromClass "/Game/Blueprints/Weapons/GrappleHook.GrappleHook_C" _returnvalue "Undefined" 0 0)))
    (:then_4
      (bind _returnvalue_4 (Game|SpawnActorfromClass "/Game/Blueprints/Player/ItemBag.ItemBag_C" _returnvalue "Undefined" 0 0))
      (Variables|Default|SetItemBag _returnvalue_4))
    (:then_5
      (bind _returnvalue_5 (Game|SpawnActorfromClass "/Game/Blueprints/UI_Elements/RightHandUI.RightHandUI_C" _returnvalue "Undefined" 0 0))
      (bind _output_get (Variables|Default|SetRightUI _returnvalue_5))
      (bind _asright_hand (Utilities|Casting|CastToRightHand (Variables|/Script/Engine.ChildActorComponent|GetChildActor (Variables|Default|GetRightHand))))
      (Transformation|AttachComponentToComponent _output_get (Variables|/Game/Blueprints/Player/Hands/RightHand.RightHand_C|Getr_hand_skeletal_lowres _asright_hand) "r_ui" "SnapToTarget" "SnapToTarget" "SnapToTarget" true))))

(event EventTick
  (params (DeltaSeconds :type Float%20%28single-precision%29))
  (if (not (!= (Variables|Default|GetMenu) 0))
    (Utilities|FlowControl|Sequence
      (:then_0
        (CallFunction|SetJoystickDirection))
      (:then_1
        (switch Utilities|FlowControl|Switch|SwitchonJoystickDirection (Variables|Default|GetJoystickDirection)
          (:NewEnumerator5
            (bind _returnvalue (Game|SpawnActorfromClass "/Game/Blueprints/UI_Elements/Menu/MenuBase.MenuBase_C" (Transformation|GetActorTransform) "Undefined" 0 0))
            (bind _output_get (Variables|Default|SetMenu _returnvalue))
            (bind _asmenu_base (Utilities|Casting|CastToMenuBase _output_get))
            (bind _holdingboworarrow (CallFunction|HasBoworArrow))
            (if _holdingboworarrow
              (Variables|/Game/Blueprints/UI_Elements/Menu/MenuBase.MenuBase_C|SetCurrentMenu _asmenu_base "NewEnumerator4")
              (Variables|/Game/Blueprints/UI_Elements/Menu/MenuBase.MenuBase_C|SetCurrentDraw _asmenu_base "NewEnumerator2")
              (else
                (Variables|/Game/Blueprints/UI_Elements/Menu/MenuBase.MenuBase_C|SetCurrentMenu _asmenu_base "NewEnumerator3")
                (Variables|/Game/Blueprints/UI_Elements/Menu/MenuBase.MenuBase_C|SetCurrentDraw _asmenu_base "NewEnumerator2")))
            (bind _asleft_hand (Utilities|Casting|CastToLeftHand (Variables|/Script/Engine.ChildActorComponent|GetChildActor (Variables|Default|GetLeftHand))))
            (Transformation|AttachComponentToComponent _output_get (Variables|/Game/Blueprints/Player/Hands/LeftHand.LeftHand_C|Getl_hand_skeletal_lowres _asleft_hand) "l_menu_socket" "SnapToTarget" "SnapToTarget" "SnapToTarget" true))
          (:NewEnumerator6
            (bind _returnvalue_2 (Game|SpawnActorfromClass "/Game/Blueprints/UI_Elements/Menu/MenuBase.MenuBase_C" (Transformation|GetActorTransform) "Undefined" 0 0))
            (bind _output_get_2 (Variables|Default|SetMenu _returnvalue_2))
            (bind _asmenu_base_2 (Utilities|Casting|CastToMenuBase _output_get_2))
            (bind _holdingboworarrow_2 (CallFunction|HasBoworArrow))
            (if _holdingboworarrow_2
              (Variables|/Game/Blueprints/UI_Elements/Menu/MenuBase.MenuBase_C|SetCurrentMenu _asmenu_base_2 "NewEnumerator5")
              (Variables|/Game/Blueprints/UI_Elements/Menu/MenuBase.MenuBase_C|SetCurrentDraw _asmenu_base_2 "NewEnumerator2")
              (else
                (Variables|/Game/Blueprints/UI_Elements/Menu/MenuBase.MenuBase_C|SetCurrentMenu _asmenu_base_2 "NewEnumerator2")
                (Variables|/Game/Blueprints/UI_Elements/Menu/MenuBase.MenuBase_C|SetCurrentDraw _asmenu_base_2 "NewEnumerator2")))
            (bind _asleft_hand_2 (Utilities|Casting|CastToLeftHand (Variables|/Script/Engine.ChildActorComponent|GetChildActor (Variables|Default|GetLeftHand))))
            (Transformation|AttachComponentToComponent _output_get_2 (Variables|/Game/Blueprints/Player/Hands/LeftHand.LeftHand_C|Getl_hand_skeletal_lowres _asleft_hand_2) "l_menu_socket" "SnapToTarget" "SnapToTarget" "SnapToTarget" true))
          (:NewEnumerator7
            (bind _returnvalue_3 (Game|SpawnActorfromClass "/Game/Blueprints/UI_Elements/Menu/MenuBase.MenuBase_C" (Transformation|GetActorTransform) "Undefined" 0 0))
            (bind _output_get_3 (Variables|Default|SetMenu _returnvalue_3))
            (bind _asmenu_base_3 (Utilities|Casting|CastToMenuBase _output_get_3))
            (Variables|/Game/Blueprints/UI_Elements/Menu/MenuBase.MenuBase_C|SetCurrentMenu _asmenu_base_3 "NewEnumerator9")
            (Variables|/Game/Blueprints/UI_Elements/Menu/MenuBase.MenuBase_C|SetCurrentDraw _asmenu_base_3 "NewEnumerator2")
            (bind _asleft_hand_3 (Utilities|Casting|CastToLeftHand (Variables|/Script/Engine.ChildActorComponent|GetChildActor (Variables|Default|GetLeftHand))))
            (Transformation|AttachComponentToComponent _output_get_3 (Variables|/Game/Blueprints/Player/Hands/LeftHand.LeftHand_C|Getl_hand_skeletal_lowres _asleft_hand_3) "l_menu_socket" "SnapToTarget" "SnapToTarget" "SnapToTarget" true))
          (:NewEnumerator8
            (bind _returnvalue_4 (Game|SpawnActorfromClass "/Game/Blueprints/UI_Elements/Menu/MenuBase.MenuBase_C" (Transformation|GetActorTransform) "Undefined" 0 0))
            (bind _output_get_4 (Variables|Default|SetMenu _returnvalue_4))
            (bind _asmenu_base_4 (Utilities|Casting|CastToMenuBase _output_get_4))
            (Variables|/Game/Blueprints/UI_Elements/Menu/MenuBase.MenuBase_C|SetCurrentMenu _asmenu_base_4 "NewEnumerator7")
            (Variables|/Game/Blueprints/UI_Elements/Menu/MenuBase.MenuBase_C|SetCurrentDraw _asmenu_base_4 "NewEnumerator2")
            (bind _asleft_hand_4 (Utilities|Casting|CastToLeftHand (Variables|/Script/Engine.ChildActorComponent|GetChildActor (Variables|Default|GetLeftHand))))
            (Transformation|AttachComponentToComponent _output_get_4 (Variables|/Game/Blueprints/Player/Hands/LeftHand.LeftHand_C|Getl_hand_skeletal_lowres _asleft_hand_4) "l_menu_socket" "SnapToTarget" "SnapToTarget" "SnapToTarget" true)))))))

(event Input|GamepadEvents|GamepadSpecialRight
  (params (Key :type Key%20Structure))
  (:Released
    (if (not (!= (Variables|Default|GetMenu) 0))
      (bind _returnvalue (Game|SpawnActorfromClass "/Game/Blueprints/UI_Elements/Menu/MenuBase.MenuBase_C" (Transformation|GetActorTransform) "Undefined" 0 0))
      (bind _output_get (Variables|Default|SetMenu _returnvalue))
      (bind _asleft_hand (Utilities|Casting|CastToLeftHand (Variables|/Script/Engine.ChildActorComponent|GetChildActor (Variables|Default|GetLeftHand))))
      (Transformation|AttachComponentToComponent _output_get (Variables|/Game/Blueprints/Player/Hands/LeftHand.LeftHand_C|Getl_hand_skeletal_lowres _asleft_hand) "l_menu_socket" "SnapToTarget" "SnapToTarget" "SnapToTarget" true))))

(fn ConstructionScript)

(fn GetInventoryCategory
  (params (Category :type InventoryCategories%20Enum :default "NewEnumerator0"))
  (bind _inventory (Variables|Default|GetInventory))
  (bind (_swords _shields _bows _arrows _bombs _boomerangs _potions) (Utilities|Struct|BreakInventory _inventory))
  (switch Utilities|FlowControl|Switch|SwitchonInventoryCategories Category
    (:NewEnumerator0
      (return _swords))
    (:NewEnumerator1
      (return _shields))
    (:NewEnumerator2
      (return _bows))
    (:NewEnumerator3
      (return _arrows))
    (:NewEnumerator5
      (return _bombs))
    (:NewEnumerator6
      (return _boomerangs))
    (:NewEnumerator4
      (return _potions))))

(fn SetInventoryCategory
  (params (Category :type InventoryCategories%20Enum :default "NewEnumerator0") (Item :type Actor%20Class%20Reference) (Index :type Integer))
  (bind _inventory (Variables|Default|GetInventory))
  (bind (_swords _shields _bows _arrows _bombs _boomerangs _potions) (Utilities|Struct|BreakInventory _inventory))
  (Utilities|FlowControl|Sequence
    (:then_0
      (LocalVariables|SetNewItem Item)
      (LocalVariables|SetNewIndex Index)
      (switch Utilities|FlowControl|Switch|SwitchonInventoryCategories Category
        (:NewEnumerator0
          (if (== (Utilities|Array|Get(acopy) _swords (LocalVariables|GetNewIndex)) 0)
            (Utilities|Array|SetArrayElem _swords (LocalVariables|GetNewIndex) (LocalVariables|GetNewItem))
            (LocalVariables|SetReplaced true)))
        (:NewEnumerator1
          (if (== (Utilities|Array|Get(acopy) _shields (LocalVariables|GetNewIndex)) 0)
            (Utilities|Array|SetArrayElem _shields (LocalVariables|GetNewIndex) (LocalVariables|GetNewItem))
            (LocalVariables|SetReplaced true)))
        (:NewEnumerator2
          (if (== (Utilities|Array|Get(acopy) _bows (LocalVariables|GetNewIndex)) 0)
            (Utilities|Array|SetArrayElem _bows (LocalVariables|GetNewIndex) (LocalVariables|GetNewItem))
            (LocalVariables|SetReplaced true)))
        (:NewEnumerator3
          (if (== (Utilities|Array|Get(acopy) _arrows (LocalVariables|GetNewIndex)) 0)
            (Utilities|Array|SetArrayElem _arrows (LocalVariables|GetNewIndex) (LocalVariables|GetNewItem))
            (LocalVariables|SetReplaced true)))
        (:NewEnumerator5
          (if (== (Utilities|Array|Get(acopy) _bombs (LocalVariables|GetNewIndex)) 0)
            (Utilities|Array|SetArrayElem _bombs (LocalVariables|GetNewIndex) (LocalVariables|GetNewItem))
            (LocalVariables|SetReplaced true)))
        (:NewEnumerator6
          (if (== (Utilities|Array|Get(acopy) _boomerangs (LocalVariables|GetNewIndex)) 0)
            (Utilities|Array|SetArrayElem _boomerangs (LocalVariables|GetNewIndex) (LocalVariables|GetNewItem))
            (LocalVariables|SetReplaced true)))
        (:NewEnumerator4
          (if (== (Utilities|Array|Get(acopy) _potions (LocalVariables|GetNewIndex)) 0)
            (Utilities|Array|SetArrayElem _potions (LocalVariables|GetNewIndex) (LocalVariables|GetNewItem))
            (LocalVariables|SetReplaced true)))))
    (:then_1
      (return (LocalVariables|GetReplaced)))))

(fn GetEquippedCategory
  (params (Category :type InventoryCategories%20Enum :default "NewEnumerator0"))
  (bind _equipped (Variables|Default|GetEquipped))
  (bind (_sword _shield _bow _arrow _bomb _boomerang _potion) (Utilities|Struct|BreakEquipped _equipped))
  (switch Utilities|FlowControl|Switch|SwitchonInventoryCategories Category
    (:NewEnumerator0
      (return _sword))
    (:NewEnumerator1
      (return _shield))
    (:NewEnumerator2
      (return _bow))
    (:NewEnumerator3
      (return _arrow))
    (:NewEnumerator5
      (return _bomb))
    (:NewEnumerator6
      (return _boomerang))
    (:NewEnumerator4
      (return _potion))))

(fn SetEquippedCategory
  (params (Category :type InventoryCategories%20Enum :default "NewEnumerator0") (Index :type Integer))
  (Utilities|FlowControl|Sequence
    (:then_0
      (LocalVariables|SetSwordIndex (.Sword (Utilities|Struct|BreakEquipped (Variables|Default|GetEquipped)))))
    (:then_1
      (LocalVariables|SetShieldIndex (.Shield (Utilities|Struct|BreakEquipped (Variables|Default|GetEquipped)))))
    (:then_2
      (LocalVariables|SetBowIndex (.Bow (Utilities|Struct|BreakEquipped (Variables|Default|GetEquipped)))))
    (:then_3
      (LocalVariables|SetArrowIndex (.Arrow (Utilities|Struct|BreakEquipped (Variables|Default|GetEquipped)))))
    (:then_4
      (LocalVariables|SetBombIndex (.Bomb (Utilities|Struct|BreakEquipped (Variables|Default|GetEquipped)))))
    (:then_5
      (LocalVariables|SetBoomerangIndex (.Boomerang (Utilities|Struct|BreakEquipped (Variables|Default|GetEquipped)))))
    (:then_6
      (LocalVariables|SetPotionIndex (.Potion (Utilities|Struct|BreakEquipped (Variables|Default|GetEquipped)))))
    (:then_7
      (switch Utilities|FlowControl|Switch|SwitchonInventoryCategories Category
        (:NewEnumerator0
          (LocalVariables|SetSwordIndex Index))
        (:NewEnumerator1
          (LocalVariables|SetShieldIndex Index))
        (:NewEnumerator2
          (LocalVariables|SetBowIndex Index))
        (:NewEnumerator3
          (LocalVariables|SetArrowIndex Index))
        (:NewEnumerator5
          (LocalVariables|SetBombIndex Index))
        (:NewEnumerator6
          (LocalVariables|SetBoomerangIndex Index))
        (:NewEnumerator4
          (LocalVariables|SetPotionIndex Index))))
    (:then_8
      (Variables|Default|SetEquipped (Utilities|Struct|MakeEquipped (LocalVariables|GetSwordIndex) (LocalVariables|GetShieldIndex) (LocalVariables|GetBowIndex) (LocalVariables|GetArrowIndex) (LocalVariables|GetBombIndex) (LocalVariables|GetBoomerangIndex) (LocalVariables|GetPotionIndex))))))

(fn ClearInventoryCategory
  (params (Category :type InventoryCategories%20Enum :default "NewEnumerator0") (Index :type Integer))
  (bind _inventory (Variables|Default|GetInventory))
  (bind (_swords _shields _bows _arrows _bombs _boomerangs _potions) (Utilities|Struct|BreakInventory _inventory))
  (switch Utilities|FlowControl|Switch|SwitchonInventoryCategories Category
    (:NewEnumerator0
      (Utilities|Array|SetArrayElem _swords Index 0))
    (:NewEnumerator1
      (Utilities|Array|SetArrayElem _shields Index 0))
    (:NewEnumerator2
      (Utilities|Array|SetArrayElem _bows Index 0))
    (:NewEnumerator3
      (Utilities|Array|SetArrayElem _arrows Index 0))
    (:NewEnumerator5
      (Utilities|Array|SetArrayElem _bombs Index 0))
    (:NewEnumerator6
      (Utilities|Array|SetArrayElem _boomerangs Index 0))
    (:NewEnumerator4
      (Utilities|Array|SetArrayElem _potions Index 0))))

(fn AddItem
  (params (Item :type Actor%20Class%20Reference) (Quantity :type Integer))
  (bind _itemquantities (Variables|Default|GetItemQuantities))
  (bind (_value _returnvalue) (Utilities|Map|Find _itemquantities Item))
  (if _returnvalue
    (Utilities|Map|Add _itemquantities Item (+ _value Quantity))
    (return false)
    (else
      (Utilities|Map|Add _itemquantities Item Quantity)
      (return true))))

(fn RemoveItem
  (params (Item :type Actor%20Class%20Reference) (Quantity :type Integer))
  (bind _itemquantities (Variables|Default|GetItemQuantities))
  (bind _itemquantities_2 (Variables|Default|GetItemQuantities))
  (bind (_value _returnvalue) (Utilities|Map|Find _itemquantities Item))
  (if _returnvalue
    (bind _output_get (LocalVariables|SetNewQuantity (- _value Quantity)))
    (if (>= _output_get 0)
      (Utilities|Map|Add _itemquantities_2 Item (LocalVariables|GetNewQuantity))
      (if (== (LocalVariables|GetNewQuantity) 0)
        ;[1 1 1] May need to make an exception for rupees
        (Utilities|Map|Remove _itemquantities_2 Item)
        ;[1 1 1] Removed all of the items remaining
        (return true true)
        (else
          ;[1 1 1] Removed some items, but there's still more!
          (return false true)))
      (else
        ;[1 1 1] Tried taking out more items than you have
        (return false false)))
    (else
      ;[1 1 1] This item doesn't exist
      (return true false))))

(fn ItemQuantity
  (params (Item :type Actor%20Class%20Reference))
  (bind _itemquantities (Variables|Default|GetItemQuantities))
  (bind (_value _returnvalue) (Utilities|Map|Find _itemquantities Item))
  (if _returnvalue
    (return _value)
    (else
      (return -1))))

(fn GetStat
  (params (Stat :type Stats%20Enum :default "NewEnumerator0"))
  (bind _stats (Variables|Default|GetStats))
  (bind (_maxhealth _health _maxmoney _money) (Utilities|Struct|BreakPlayerStats _stats))
  (switch Utilities|FlowControl|Switch|SwitchonStats Stat
    (:NewEnumerator0
      (return _maxhealth))
    (:NewEnumerator1
      (return _health))
    (:NewEnumerator2
      (return _maxmoney))
    (:NewEnumerator3
      (return _money))))

(fn SetStat
  (params (Stat :type Stats%20Enum :default "NewEnumerator0") (Value :type Integer))
  (Utilities|FlowControl|Sequence
    (:then_0
      (LocalVariables|SetMaxHealth (.MaxHealth (Utilities|Struct|BreakPlayerStats (Variables|Default|GetStats)))))
    (:then_1
      (LocalVariables|SetHealth (.Health (Utilities|Struct|BreakPlayerStats (Variables|Default|GetStats)))))
    (:then_2
      (LocalVariables|SetMaxMoney (.MaxMoney (Utilities|Struct|BreakPlayerStats (Variables|Default|GetStats)))))
    (:then_3
      (LocalVariables|SetMoney (.Money (Utilities|Struct|BreakPlayerStats (Variables|Default|GetStats)))))
    (:then_6
      (switch Utilities|FlowControl|Switch|SwitchonStats Stat
        (:NewEnumerator0
          (LocalVariables|SetMaxHealth Value))
        (:NewEnumerator1
          (LocalVariables|SetHealth (Math|Integer|Clamp(Integer) Value 0 (LocalVariables|GetMaxHealth))))
        (:NewEnumerator2
          (LocalVariables|SetMaxMoney Value))
        (:NewEnumerator3
          (LocalVariables|SetMoney (Math|Integer|Clamp(Integer) Value 0 (LocalVariables|GetMaxMoney))))))
    (:then_7
      (Variables|Default|SetStats (Utilities|Struct|MakePlayerStats (LocalVariables|GetMaxHealth) (LocalVariables|GetHealth) (LocalVariables|GetMaxMoney) (LocalVariables|GetMoney))))))

(fn AddStat
  (params (Stat :type Stats%20Enum :default "NewEnumerator0") (Amount :type Integer))
  (bind _resultstat (CallFunction|GetStat Stat))
  (if (< (+ _resultstat Amount) 0)
    (return _resultstat false)
    (else
      (CallFunction|SetStat Stat (+ _resultstat Amount))
      (bind _resultstat_2 (CallFunction|GetStat Stat))
      (return _resultstat_2 true))))

(fn HasBoworArrow
  (Utilities|FlowControl|Sequence
    (:then_0
      (bind _asleft_hand (Utilities|Casting|CastToLeftHand (Variables|/Script/Engine.ChildActorComponent|GetChildActor (Variables|Default|GetLeftHand))))
      (for _array_element (Actor|GetAttachedActors _asleft_hand)
        (if (or (Utilities|DoesObjectImplementInterface _array_element "/Game/Blueprints/Interfaces/Arrow.Arrow_C") (Utilities|DoesObjectImplementInterface _array_element "/Game/Blueprints/Interfaces/Bow.Bow_C"))
          (LocalVariables|SetDoesIt? true))))
    (:then_1
      (bind _asright_hand (Utilities|Casting|CastToRightHand (Variables|/Script/Engine.ChildActorComponent|GetChildActor (Variables|Default|GetRightHand))))
      (for _array_element_2 (Actor|GetAttachedActors _asright_hand)
        (if (or (Utilities|DoesObjectImplementInterface _array_element_2 "/Game/Blueprints/Interfaces/Arrow.Arrow_C") (Utilities|DoesObjectImplementInterface _array_element_2 "/Game/Blueprints/Interfaces/Bow.Bow_C"))
          (LocalVariables|SetDoesIt? true))))
    (:then_2
      (return (LocalVariables|GetDoesIt?)))))

(fn SetJoystickDirection
  (bind _returnvalue (Class|Actor|GetInputAxisKeyValue))
  (bind _returnvalue_2 (Class|Actor|GetInputAxisKeyValue))
  (if (< _returnvalue -0.5)
    (Variables|Default|SetJoystickDirection "NewEnumerator0")
    (elif (> _returnvalue 0.5)
      (Variables|Default|SetJoystickDirection "NewEnumerator1")
      (elif (< _returnvalue_2 -0.5)
        (Variables|Default|SetJoystickDirection "NewEnumerator2")
        (elif (> _returnvalue_2 0.5)
          (Variables|Default|SetJoystickDirection "NewEnumerator3")
          (else
            (switch Utilities|FlowControl|Switch|SwitchonJoystickDirection (Variables|Default|GetJoystickDirection)
              (:NewEnumerator4
                (Variables|Default|SetJoystickDirection "NewEnumerator4"))
              (:NewEnumerator0
                (Variables|Default|SetJoystickDirection "NewEnumerator5"))
              (:NewEnumerator1
                (Variables|Default|SetJoystickDirection "NewEnumerator6"))
              (:NewEnumerator2
                (Variables|Default|SetJoystickDirection "NewEnumerator7"))
              (:NewEnumerator3
                (Variables|Default|SetJoystickDirection "NewEnumerator8"))
              (:NewEnumerator5
                (Variables|Default|SetJoystickDirection "NewEnumerator4" :!label _label))
              (:NewEnumerator6
                (goto _label))
              (:NewEnumerator7
                (goto _label))
              (:NewEnumerator8
                (goto _label)))))))))