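; ItemBag is a player item bag actor that keeps itself at a fixed spot relative to the player's view.
; Each Tick teleports its Origin component to the camera manager's X and Y at the pawn's height, matching only camera yaw.
; It then applies a constant local offset and rotation to the actor, so the bag follows turning while ignoring camera pitch and roll.
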(event EventTick
  (params (DeltaSeconds :type Float%20%28single-precision%29))
  (bind _returnvalue (Game|GetPlayerCameraManager 0))
  (bind _returnvalue_2 (Transformation|GetActorTransform _returnvalue))
  (bind (_location _rotation) (Math|Transform|BreakTransform _returnvalue_2))
  (bind (_x _y) (Math|Vector|BreakVector _location))
  (Utilities|FlowControl|Sequence
    (:then_0
      (Transformation|SetWorldLocationAndRotation (Variables|Default|GetOrigin) (Math|Vector|MakeVector _x _y (.Z (Math|Vector|BreakVector (Transformation|GetActorLocation (Game|Player|GetPlayerPawn 0))))) (Math|Rotator|MakeRotator 0.0 0.0 (.Yaw (Math|Rotator|BreakRotator _rotation))) false true)
      (Transformation|AddActorLocalOffset "0.000000,-25.000000,80.000000" false false)
      (Transformation|AddActorLocalRotation "0.000000,-110.000000,45.000000" false false))))

(fn ConstructionScript)